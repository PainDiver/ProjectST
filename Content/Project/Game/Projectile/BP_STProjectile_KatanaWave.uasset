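; Katana wave projectile that damages actors it overlaps, reporting hits through the game state.
; On the authority, sphere overlaps with anything but the instigator register a hit message with a fixed hit parameter index, without stopping the projectile.
; Authority Tick measures distance from the spawn location and, at the travel limit, flags pending destroy, deactivates the particles and disables sphere collision.
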(event OnComponentBeginOverlap(Sphere)
  (params (OverlappedComponent :type Primitive%20Component%20Object%20Reference) (OtherActor :type Actor%20Object%20Reference) (OtherComp :type Primitive%20Component%20Object%20Reference) (OtherBodyIndex :type Integer) (bFromSweep :type Boolean) (SweepResult :type Hit%20Result%20Structure%20%28by%20ref%29))
  (if (!= (Game|GetInstigator) OtherActor)
    (Networking|SwitchHasAuthority
      (:Authority
        (Class|IBPSTGameState|RegisterHit(Message) (Game|GetGameState) (Game|GetInstigator) OtherActor 16)))))

(event Custom|OnDeactivate
  (Variables|Default|SetPendingDestroy true)
  (Components|Activation|Deactivate (Variables|Default|GetParticleSystem))
  (Collision|SetCollisionEnabled (Variables|Default|GetSphere) "NoCollision"))

(event EventBeginPlay
  (Variables|Default|SetInitialLocation (Transformation|GetActorLocation)))

(event Collision|EventActorBeginOverlap
  (params (OtherActor :type Actor%20Object%20Reference)))

(event EventTick
  (params (DeltaSeconds :type Float%20%28single-precision%29))
  (if (Ability|HasAuthority)
    (if (>= (Math|Vector|Distance(Vector) (Variables|Default|GetInitialLocation) (Transformation|GetActorLocation)) (Variables|Default|GetTravelDistance))
      (CallFunction|OnDeactivate))))

(fn ConstructionScript)