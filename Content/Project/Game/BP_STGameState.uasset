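; BP_STGameState is a game state that arbitrates combat hits, holding them briefly to catch simultaneous trades.
; RegisterHit queues hits on non-immortal defenders, unless a pending hit against the attacker has the same HitType in HitParamTable.
; Such pairs cancel out, since ProcessSimultaneousHit is a stub.
; On authority, Tick flushes hits older than HitFlushTime, activating the defender's GAS hit ability and sending it a gameplay event.
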(event EventBeginPlay)

(event EventTick
  (params (DeltaSeconds :type Float%20%28single-precision%29))
  (Networking|SwitchHasAuthority
    (:Authority
      (CallFunction|FlushHits))))

(fn ConstructionScript)

(fn FindSimultaneousHit
  (params (Attacker :type Actor%20Object%20Reference) (HitParamIndex :type Integer))
  (bind _output_get (LocalVariables|SetLocalDelayedHits (Variables|Default|GetDelayedHits)))
  (for _array_element _output_get
    (LocalVariables|SetLocalCurrentHit _array_element)
    (if (== Attacker (.Defender (Utilities|Struct|BreakHitInfo _array_element)))
      (bind _returnvalue (Utilities|GetDataTableRow "/Game/Project/TableData/HitParamTable.HitParamTable" (Utilities|String|StringToName (Utilities|String|ToString(Integer) (.HitInfoIndex (Utilities|Struct|BreakHitInfo _array_element)))))
        (:then
          (bind _returnvalue_2 (Utilities|GetDataTableRow "/Game/Project/TableData/HitParamTable.HitParamTable" (Utilities|String|StringToName (Utilities|String|ToString(Integer) HitParamIndex)))
            (:then
              (if (== (.HitType (Utilities|Struct|BreakHitParam _returnvalue_2)) (.HitType (Utilities|Struct|BreakHitParam _returnvalue)))
                (Utilities|Array|RemoveItem (Variables|Default|GetDelayedHits) (LocalVariables|GetLocalCurrentHit))
                (return true (LocalVariables|GetLocalCurrentHit))))))))))

(fn FlushHits
  (if (> (Utilities|Array|Length (Variables|Default|GetDelayedHits)) 0)
    (bind _output_get (LocalVariables|SetLocalHits (Variables|Default|GetDelayedHits)))
    (for _array_element _output_get
      (LocalVariables|SetLocalCurrentHitInfo _array_element)
      (if (> (- (Utilities|Time|GetTimeSeconds) (.TimeStamp (Utilities|Struct|BreakHitInfo _array_element))) (Variables|Default|GetHitFlushTime))
        (Utilities|Array|RemoveItem (Variables|Default|GetDelayedHits) (LocalVariables|GetLocalCurrentHitInfo))
        (CallFunction|ProcessHit (LocalVariables|GetLocalCurrentHitInfo))))))

(fn ProcessHit
  (params (HitInfo :type Hit%20Info%20Structure))
  (bind (_defender _dataifset) (Utilities|Struct|BreakHitInfo HitInfo))
  (bind (_attacker _defender_2 _hitinfoindex) (Utilities|Struct|BreakHitInfo HitInfo))
  (bind (_eventtag _instigator _target _optionalobject _optionalobject2 _contexthandle _instigatortags _targettags _eventmagnitude _targetdata) (Utilities|Struct|BreakGameplayEventData _dataifset))
  (bind _returnvalue (Abilities|TryActivateAbilitybyClass (Ability|GetAbilitySystemComponent (.Defender (Utilities|Struct|BreakHitInfo HitInfo))) "/Game/Project/GAS/Action/BP_STGA_Hit.BP_STGA_Hit_C" false))
  (if _returnvalue
    (bind _returnvalue_2 (Game|ConstructObjectfromClass _defender_2 "/Game/Project/GAS/Action/BP_HitInfoObject.BP_HitInfoObject_C" _hitinfoindex))
    (Ability|SendGameplayEventtoActor _defender "(TagName=\"GA.Action.Hit\")" (Utilities|Struct|MakeGameplayEventData _eventtag _attacker _defender_2 _returnvalue_2 _optionalobject2 _contexthandle _instigatortags _targettags _eventmagnitude _targetdata))
    (return true)
    (else
      (return false))))

(fn ProcessSimultaneousHit
  (params (PreviousHit :type Hit%20Info%20Structure) (NewHit :type Hit%20Info%20Structure))
  (return true))

(fn RegisterHit
  (params (Attacker :type Actor%20Object%20Reference) (Defender :type Actor%20Object%20Reference) (HitParamIndex :type Integer) (EventDataIfSet :type Gameplay%20Event%20Data%20Structure))
  (bind _returnvalue (Class|STStateInterface|IsImmortalState(Message) Defender))
  (if (not _returnvalue)
    (if (!= HitParamIndex 0)
      (LocalVariables|SetLocalNewHitInfo (Utilities|Struct|MakeHitInfo Attacker Defender HitParamIndex (Utilities|Time|GetTimeSeconds) EventDataIfSet))
      (bind (_res _prehitinfo) (CallFunction|FindSimultaneousHit Attacker HitParamIndex))
      (if _res
        (CallFunction|ProcessSimultaneousHit _prehitinfo (LocalVariables|GetLocalNewHitInfo))
        (else
          (Utilities|Array|Add (Variables|Default|GetDelayedHits) (LocalVariables|GetLocalNewHitInfo)))))))