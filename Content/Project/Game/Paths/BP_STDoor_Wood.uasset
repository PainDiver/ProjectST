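; Breakable wooden door for a networked game that gives wood-particle and impact-sound feedback when hit and shatters when destroyed.
; STDestruction delegates drive it: non-dedicated instances play effects and add a geometry collection, while the dedicated server destroys the actor after a delay.
; A separate OnGetAttacked path decrements BreakCount and calls GetDamaged, which runs similar remote-only effects and removes the debris after a delay.
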(event Custom|GetDamaged
  (params (BreakCount :type Integer))
  (bind _cube (Variables|Default|GetCube))
  (bind _returnvalue (Transformation|GetWorldLocation _cube))
  (Networking|SwitchHasAuthority
    (:Remote
      (Effects|SpawnEmitteratLocation "/Game/ExternalResource/Realistic_Starter_VFX_Pack_Vol2/Particles/Hit/P_Wood.P_Wood" _returnvalue "0, 0, 0" "3.000000,3.000000,3.000000")
      (Audio|PlaySoundatLocation "/Game/ExternalResource/Free_Sounds_Pack/wav/Rock_Impact_11.Rock_Impact_11" _returnvalue "0, 0, 0" 1.0 1.0 0.0 0 0 0 0)
      (if (<= BreakCount 0)
        (Components|DestroyComponent (Variables|Default|GetCube))
        (bind _returnvalue_2 (AddComponent|AddGeometryCollectionComponent false))
        (Utilities|FlowControl|Delay 3.0)
        (Components|DestroyComponent _returnvalue_2)))))

(event Custom|OnDestructionDelegate_이벤트
  (Components|DestroyComponent (Variables|Default|GetCube))
  (if (Networking|IsDedicatedServer)
    (Utilities|FlowControl|Delay 3.0)
    (Actor|DestroyActor)
    (else
      (AddComponent|AddGeometryCollectionComponent false))))

(event Custom|OnDamageDelegate_이벤트
  (params (Damage :type Integer))
  (bind _cube (Variables|Default|GetCube))
  (bind _returnvalue (Transformation|GetWorldLocation _cube))
  (if (not (Networking|IsDedicatedServer))
    (Effects|SpawnEmitteratLocation "/Game/ExternalResource/Realistic_Starter_VFX_Pack_Vol2/Particles/Hit/P_Wood.P_Wood" _returnvalue "0, 0, 0" "3.000000,3.000000,3.000000")
    (Audio|PlaySoundatLocation "/Game/ExternalResource/Free_Sounds_Pack/wav/Rock_Impact_11.Rock_Impact_11" _returnvalue "0, 0, 0" 1.0 1.0 0.0 0 0 0 0)))

(event EventBeginPlay
  (|CallParentFunction)
  (EventDispatchers|AssignOnDamageDelegate (Variables|Default|GetSTDestruction) (delegate Custom|OnDamageDelegate_이벤트))
  (EventDispatchers|AssignOnDestructionDelegate (Variables|Default|GetSTDestruction) (delegate Custom|OnDestructionDelegate_이벤트)))

(event Collision|EventActorBeginOverlap
  (params (OtherActor :type Actor%20Object%20Reference))
  (|CallParentFunction OtherActor) ; 지금 이 노드는 비활성 상태입니다. \n핀을 끌어서 다른 노드를 연결하면 활성화됩니다.
)

(event EventTick
  (params (DeltaSeconds :type Float%20%28single-precision%29))
  (|CallParentFunction DeltaSeconds) ; 지금 이 노드는 비활성 상태입니다. \n핀을 끌어서 다른 노드를 연결하면 활성화됩니다.
)

(event EventOnGetAttacked
  (params (BreakDamage :type Integer))
  (bind _result (Math|Integer|DecrementInt (Variables|Default|GetBreakCount))
    (:%20%20
      (CallFunction|GetDamaged _result)
      (if (<= (Variables|Default|GetBreakCount) 0)
        (Components|DestroyComponent (Variables|Default|GetCube))))))

(fn ConstructionScript
  (|CallParentFunction))