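; Interactable, damageable swing door that opens away from the character using it.
; BeginPlay binds interaction delegates on STInteractionObject; a successful interaction plays a push montage and compares the interactor's direction against forward and backward arrows.
; A closed door swings open that way; an open one closes from the opposite direction or over-opens from the same one.
; Timelines drive the Scene component's yaw, while attacks pass damage to STDestruction.
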(event Custom|OpenDoor
  (params (IsForward :type Boolean))
  (Variables|Default|SetLastIsForward IsForward)
  (bind _새_트랙_0 (Timeline|OpenDoorAnim PlayFromStart)
    (:Update
      (bind _output_get (Variables|Default|SetLastDoorRot (* _새_트랙_0 (select IsForward -1.0 1.0))))
      (Transformation|SetRelativeRotation (Variables|Default|GetScene) (Math|Rotator|MakeRotator 0.0 0.0 _output_get) false false))
    (:Finished
      (Variables|Default|SetIsOpen true))))

(event Custom|CloseDoor
  (bind _새_트랙_0 (Timeline|CloseDoorAnim PlayFromStart)
    (:Update
      (bind _output_get (Variables|Default|SetLastDoorRot (* _새_트랙_0 (select (Variables|Default|GetLastIsForward) -1.0 1.0))))
      (Transformation|SetRelativeRotation (Variables|Default|GetScene) (Math|Rotator|MakeRotator 0.0 0.0 _output_get) false false))
    (:Finished
      (Variables|Default|SetIsOpen false))))

(event Custom|OverOpen
  (bind _새_트랙_0 (Timeline|OverOpenAnim PlayFromStart)
    (:Update
      (bind _output_get (Variables|Default|SetLastDoorRot (* _새_트랙_0 (select (Variables|Default|GetLastIsForward) -1.0 1.0))))
      (Transformation|SetRelativeRotation (Variables|Default|GetScene) (Math|Rotator|MakeRotator 0.0 0.0 _output_get) false false))))

(event EventBeginPlay
  (|CallParentFunction)
  (CallFunction|BindEvent))

(event Collision|EventActorBeginOverlap
  (params (OtherActor :type Actor%20Object%20Reference))
  (|CallParentFunction OtherActor) ; 지금 이 노드는 비활성 상태입니다. \n핀을 끌어서 다른 노드를 연결하면 활성화됩니다.
)

(event EventTick
  (params (DeltaSeconds :type Float%20%28single-precision%29))
  (|CallParentFunction DeltaSeconds) ; 지금 이 노드는 비활성 상태입니다. \n핀을 끌어서 다른 노드를 연결하면 활성화됩니다.
)

(event EventOnGetAttacked
  (params (BreakDamage :type Integer))
  (Class|STDestructionComponent|DamageObject (Variables|Default|GetSTDestruction) BreakDamage))

(fn ConstructionScript
  (|CallParentFunction))

(fn BindEvent
  (|SetBy-RefVar (Utilities|Array|Get(acopy) (Variables|/Script/ProjectST.STInteractionObjectComponent|GetInteractionDelegates (Variables|Default|GetSTInteractionObject))) (Utilities|Struct|MakeInteractionDelegateSets (EventDispatchers|CreateEvent :!event CanInteract) (EventDispatchers|CreateEvent :!event OnStartInteraction) "(null).None" "(null).None" (EventDispatchers|CreateEvent :!event OnEndInteraction))))

(fn CanInteract
  (params (Interactor :type Actor%20Object%20Reference) (InteractionInfo :type Interaction%20Info%20Structure%20%28by%20ref%29))
  (return true))

(fn OnStartInteraction
  (params (Interactor :type Actor%20Object%20Reference) (InteractionInfo :type Interaction%20Info%20Structure%20%28by%20ref%29)))

(fn OnEndInteraction
  (params (Interactor :type Actor%20Object%20Reference) (bIsSuccess :type Boolean) (InteractionInfo :type Interaction%20Info%20Structure%20%28by%20ref%29))
  (if bIsSuccess
    (bind _asstcharacter_base (Utilities|Casting|CastToSTCharacterBase Interactor))
    (Animation|PlayAnimMontage _asstcharacter_base "/Game/Project/Character/Animation/ProcessedAnimation/Interaction/A_Push_Montage.A_Push_Montage" 1.1 "None")
    (if (Variables|Default|GetIsOpen)
      (bind _forward (CallFunction|CalculateDirection Interactor))
      (if (!= _forward (Variables|Default|GetLastIsForward))
        (CallFunction|CloseDoor)
        (else
          (CallFunction|OverOpen)))
      (else
        (bind _forward_2 (CallFunction|CalculateDirection Interactor))
        (CallFunction|OpenDoor _forward_2)))))

(fn CalculateDirection
  (params (Interactor :type Actor%20Object%20Reference))
  (bind _output_get (LocalVariables|SetLocalInteractorToDoor (Math|Vector|Normalize (- (Transformation|GetActorLocation) (Transformation|GetActorLocation Interactor)))))
  (return (> (Class|KismetMathLibrary|VectorCosineAngle2D _output_get (Math|Vector|GetForwardVector (Variables|Default|GetForwardArrow))) (Class|KismetMathLibrary|VectorCosineAngle2D _output_get (Math|Vector|GetForwardVector (Variables|Default|GetBackwardArrow))))))