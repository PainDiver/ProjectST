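; Cheat component that adds or removes gameplay-tag states on the player pawn by tag name.
; AddState and RemoveState pass the tag and player pawn 0 to their server counterparts.
; The server events convert the name to a gameplay tag and, if it is valid, call Add or RemoveStateReplicationMessage on the pawn.
; BeginPlay and Tick are unused.
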(event Custom|RemoveState_Server
  (params (Tag :type String) (타깃 :type Object%20Object%20Reference))
  (bind _returnvalue (Utilities|String|StringToName Tag))
  (bind _returnvalue_2 (Class|STGameBlueprintFunctionLibrary|RequestGameplayTag _returnvalue))
  (if (GameplayTags|IsGameplayTagValid _returnvalue_2)
    (Class|STStateInterface|RemoveStateReplication(Message) 타깃 _returnvalue_2)))

(event Custom|AddState_Server
  (params (Tag :type String) (타깃 :type Object%20Object%20Reference))
  (bind _returnvalue (Utilities|String|StringToName Tag))
  (bind _returnvalue_2 (Class|STGameBlueprintFunctionLibrary|RequestGameplayTag _returnvalue))
  (if (GameplayTags|IsGameplayTagValid _returnvalue_2)
    (Class|STStateInterface|AddStateReplication(Message) 타깃 _returnvalue_2)))

(event Custom|RemoveState
  (params (Tag :type String))
  (CallFunction|RemoveStateServer Tag (Game|Player|GetPlayerPawn 0)))

(event Custom|AddState
  (params (Tag :type String))
  (CallFunction|AddStateServer Tag (Game|Player|GetPlayerPawn 0)))

(event EventBeginPlay)

(event EventTick
  (params (DeltaSeconds :type Float%20%28single-precision%29)))