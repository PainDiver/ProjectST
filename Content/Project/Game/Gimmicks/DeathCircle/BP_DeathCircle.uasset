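; Battle-royale death circle: a safe zone that shrinks in phases and spawns a Quinn enemy at its final center.
; PhaseComponent events select each smaller circle inside the previous target, preferring reachable navmesh points, and start the shrink.
; Tick lerps SafeArea's scale and location toward that target.
; The server applies a phase-leveled GameplayEffect to characters outside, while clients drive the HUD warning and wall material intensity.
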(event EventBeginPlay
  (CallFunction|BindInitialEvent))

(event Collision|EventActorBeginOverlap
  (params (OtherActor :type Actor%20Object%20Reference)))

(event EventTick
  (params (DeltaSeconds :type Float%20%28single-precision%29))
  (CallFunction|ProcessShrink DeltaSeconds))

(fn ConstructionScript)

(fn OnTickPhase
  (params (CurrentPhaseContext :type Phase%20Context%20Structure%20%28by%20ref%29) (PhaseInfo :type Phase%20Info%20Structure%20%28by%20ref%29))
  (Networking|SwitchHasAuthority
    (:Authority
      (bind _outactors (Actor|GetAllActorsOfClass "/Script/ProjectST.STCharacterBase"))
      (for _array_element _outactors
        (if (Collision|IsOverlappingActor (Variables|Default|GetSafeArea) _array_element :!class /Script/Engine.PrimitiveComponent)
          (if (.ReturnValue (Utilities|Map|Find (Variables|Default|GetPlayersOutOfRange) _array_element))
            (GameplayEffects|RemoveActiveGameplayEffect (Ability|GetAbilitySystemComponent _array_element) (.Value (Utilities|Map|Find (Variables|Default|GetPlayersOutOfRange) _array_element)) -1)
            (Utilities|Map|Remove (Variables|Default|GetPlayersOutOfRange) _array_element))
          (elif (not (.ReturnValue (Utilities|Map|Find (Variables|Default|GetPlayersOutOfRange) _array_element)))
            (bind _returnvalue (GameplayEffects|ApplyGameplayEffectToSelf (Ability|GetAbilitySystemComponent _array_element) "/Game/Project/GAS/Effect/BP_STGE_DeathCircle.BP_STGE_DeathCircle_C" (Math|Conversions|ToFloat(Integer) (Utilities|Struct|BreakPhaseContext CurrentPhaseContext)) (GameplayEffects|MakeEffectContext (Ability|GetAbilitySystemComponent _array_element))))
            (Utilities|Map|Add (Variables|Default|GetPlayersOutOfRange) _array_element _returnvalue)))))
    (:Remote
      (if (Collision|IsOverlappingActor (Variables|Default|GetSafeArea) (Game|Player|GetPlayerPawn 0) :!class /Script/Engine.PrimitiveComponent)
        (Class|IBPSTHUDInterface|ShowDeathCircleInterface(Message) (HUD|GetHUD (Game|GetPlayerController 0)) 0.0)
        (else
          (Class|IBPSTHUDInterface|ShowDeathCircleInterface(Message) (HUD|GetHUD (Game|GetPlayerController 0)) (+ (* (Math|Conversions|ToFloat(Integer) (Utilities|Struct|BreakPhaseContext CurrentPhaseContext)) 0.05) 0.1)))))))

(fn OnPhaseIncrement
  (params (CurrentPhaseContext :type Phase%20Context%20Structure%20%28by%20ref%29) (PhaseInfo :type Phase%20Info%20Structure%20%28by%20ref%29))
  (bind _deathcirclephaseinfo (Variables|Default|GetDeathCirclePhaseInfo))
  (bind _playersoutofrange (Variables|Default|GetPlayersOutOfRange))
  (bind _currentphase (Utilities|Struct|BreakPhaseContext CurrentPhaseContext))
  (bind _output (Utilities|Array|Get(acopy) _deathcirclephaseinfo _currentphase))
  (Variables|Default|SetIsShrinkStarted false)
  (Utilities|FlowControl|Sequence
    (:then_1
      (Networking|SwitchHasAuthority
        (:Authority
          (Utilities|FlowControl|Sequence
            (:then_0
              (bind _keys (Utilities|Map|Keys _playersoutofrange))
              (for _array_element _keys
                (GameplayEffects|SetActiveGameplayEffectLevel (Ability|GetAbilitySystemComponent _array_element) (.Value (Utilities|Map|Find _playersoutofrange _array_element)) (Utilities|Struct|BreakPhaseContext CurrentPhaseContext))))
            (:then_1
              (Variables|Default|SetTargetCenterLocation (CallFunction|PickRandomTargetLoc (Variables|Default|GetTargetCenterLocation) (Variables|Default|GetTargetRadius) (.radius _output)))
              (Variables|Default|SetTargetRadius (.radius _output)))))))))

(fn PickRandomTargetLoc
  (params (Center :type Vector%202D%20Structure) (OuterCircleRadius :type Float%20%28double-precision%29) (InnerCircleRadius :type Float%20%28double-precision%29))
  (bind _output_get (LocalVariables|SetLocalValidRadius (- OuterCircleRadius InnerCircleRadius)))
  (if (.ReturnValue (AI|Navigation|GetRandomReachablePointinRadius (Math|Conversions|ToVector(Vector2D) Center) _output_get 0 0))
    (return (Math|Conversions|ToVector2D(Vector) (.RandomLocation (AI|Navigation|GetRandomReachablePointinRadius (Math|Conversions|ToVector(Vector2D) Center) _output_get 0 0))))
    (else
      (return (+ Center (Math|Vector2D|MakeVector2D (* (LocalVariables|GetLocalValidRadius) (Math|Trig|Cos(Degrees) (Math|Random|RandomFloatinRange 0.0 3.6e+02))) (* (LocalVariables|GetLocalValidRadius) (Math|Trig|Sin(Degrees) (Math|Random|RandomFloatinRange 0.0 3.6e+02)))))))))

(fn OnPhaseShrink
  (params (CurrentPhaseContext :type Phase%20Context%20Structure%20%28by%20ref%29) (PhaseInfo :type Phase%20Info%20Structure%20%28by%20ref%29))
  (Variables|Default|SetIsShrinkStarted true)
  (Variables|Default|SetCurrentShrink%20Duration (.ShrinkDuration (Utilities|Struct|BreakPhaseInfo PhaseInfo)))
  (Variables|Default|SetElapsedTimeOnShrink 0.0))

(fn ProcessShrink
  (params (DeltaTime :type Float%20%28double-precision%29))
  (bind _targetcenterlocation (Variables|Default|GetTargetCenterLocation))
  (bind _safearea (Variables|Default|GetSafeArea))
  (bind _targetradius (Variables|Default|GetTargetRadius))
  (bind _safearea_2 (Variables|Default|GetSafeArea))
  (bind _returnvalue (Transformation|GetWorldScale _safearea))
  (bind (_x _y) (Math|Vector2D|BreakVector2D _targetcenterlocation))
  (bind _returnvalue_2 (Transformation|GetWorldLocation _safearea_2))
  (if (Variables|Default|GetIsShrinkStarted)
    (Variables|Default|SetElapsedTimeOnShrink (+ (Variables|Default|GetElapsedTimeOnShrink) DeltaTime))
    (bind _output_get (LocalVariables|SetLocalShrinkAlpha (Math|Float|Clamp(Float) (/ (Variables|Default|GetElapsedTimeOnShrink) (Variables|Default|GetCurrentShrink%20Duration)))))
    (if (>= _output_get 0.999)
      (Variables|Default|SetIsShrinkStarted false)
      (else
        (Transformation|SetWorldScale3D (Variables|Default|GetSafeArea) (Math|Vector|Lerp(Vector) _returnvalue (Math|Vector|MakeVector _targetradius _targetradius (.Z (Math|Vector|BreakVector _returnvalue))) (LocalVariables|GetLocalShrinkAlpha)))
        (Transformation|SetWorldLocation (Variables|Default|GetSafeArea) (Math|Vector|Lerp(Vector) _returnvalue_2 (Math|Vector|MakeVector _x _y (.Z (Math|Vector|BreakVector _returnvalue_2))) (LocalVariables|GetLocalShrinkAlpha)) false true)
        (Networking|SwitchHasAuthority
          (:Remote
            (bind _returnvalue_3 (Rendering|Material|GetScalarParameterValue (Variables|Default|GetDynamicMaterial) "Strength" :!class /Script/Engine.MaterialInstanceDynamic))
            (Rendering|Material|SetScalarParameterValue (Variables|Default|GetDynamicMaterial) "Strength" (Math|Float|Lerp _returnvalue_3 (Math|Conversions|ToFloat(Integer) (* (.currentphase (Variables|/Script/ProjectST.PhaseComponent|GetCurrentPhaseContext (Variables|Default|GetPhaseComponent))) 10)) (LocalVariables|GetLocalShrinkAlpha)) :!class /Script/Engine.MaterialInstanceDynamic)
            (bind _returnvalue_4 (Rendering|Material|GetScalarParameterValue (Variables|Default|GetDynamicMaterial) "Opacity" :!class /Script/Engine.MaterialInstanceDynamic))
            (Rendering|Material|SetScalarParameterValue (Variables|Default|GetDynamicMaterial) "Opacity" (Math|Float|Lerp _returnvalue_4 (Math|Float|Clamp(Float) (* (Math|Conversions|ToFloat(Integer) (.currentphase (Variables|/Script/ProjectST.PhaseComponent|GetCurrentPhaseContext (Variables|Default|GetPhaseComponent)))) 0.05) 0.1) (LocalVariables|GetLocalShrinkAlpha)) :!class /Script/Engine.MaterialInstanceDynamic)))))
    (else
      (Variables|Default|SetElapsedTimeOnShrink 0.0))))

(fn BindInitialEvent
  (bind _returnvalue (Transformation|GetActorLocation))
  (Utilities|FlowControl|Sequence
    (:then_0
      (Networking|SwitchHasAuthority
        (:Authority
          (Variables|Default|SetTargetCenterLocation (Math|Vector2D|MakeVector2D (.x _returnvalue) (.y _returnvalue)))
          (Variables|Default|SetTargetRadius (.radius (Utilities|Array|Get(acopy) (Variables|Default|GetDeathCirclePhaseInfo)))))
        (:Remote
          (bind _returnvalue_2 (Rendering|Material|CreateDynamicMaterialInstance (Variables|Default|GetSafeArea) 0 (Rendering|Material|GetMaterial (Variables|Default|GetSafeArea) 0) "None" :!class /Script/Engine.PrimitiveComponent))
          (Rendering|Material|SetMaterial (Variables|Default|GetSafeArea) 0 _returnvalue_2)
          (Variables|Default|SetDynamicMaterial _returnvalue_2))))
    (:then_1
      (EventDispatchers|BindEventtoOnPhaseTick (Variables|Default|GetPhaseComponent) (EventDispatchers|CreateEvent :!event OnTickPhase))
      (EventDispatchers|BindEventtoOnPhaseIncremented (Variables|Default|GetPhaseComponent) (EventDispatchers|CreateEvent :!event OnPhaseIncrement))
      (EventDispatchers|BindEventtoOnPhaseShrink (Variables|Default|GetPhaseComponent) (EventDispatchers|CreateEvent :!event OnPhaseShrink))
      (EventDispatchers|BindEventtoOnPhaseEnded (Variables|Default|GetPhaseComponent) (EventDispatchers|CreateEvent :!event OnPhaseEnded)))))

(fn OnPhaseEnded
  (bind _targetcenterlocation (Variables|Default|GetTargetCenterLocation))
  (Networking|SwitchHasAuthority
    (:Authority
      (bind (_outhit _returnvalue) (Collision|LineTraceByChannel (Math|Vector|MakeVector (.x _targetcenterlocation) (.y _targetcenterlocation) 2e+04) (Math|Vector|MakeVector (.x _targetcenterlocation) (.y _targetcenterlocation) -5e+04) "TraceTypeQuery1" false 0 "None"))
      (if _returnvalue
        (Game|SpawnActorfromClass "/Game/Project/Character/Enemy/BP_STEnemyCharacter_Quinn.BP_STEnemyCharacter_Quinn_C" (Math|Transform|MakeTransform (.ImpactPoint (Collision|BreakHitResult _outhit)) "0, 0, 0" "1.000000,1.000000,1.000000") "Undefined" "MultiplyWithRoot" (Game|GetGameState) 0)))))

(fn GetDeathCircleTransform
  (return (* (.X (Math|Vector|BreakVector (Transformation|GetWorldScale (Variables|Default|GetSafeArea)))) 45.0) (Transformation|GetWorldLocation (Variables|Default|GetSafeArea)) (* (Variables|Default|GetTargetRadius) 45.0) (Variables|Default|GetTargetCenterLocation)))