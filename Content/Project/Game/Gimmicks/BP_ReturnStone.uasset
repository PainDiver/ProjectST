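; BP_ReturnStone is an interactable Return Stone gimmick that animates its mesh into place on spawn and blocks interaction until the move finishes.
; BeginPlay moves the mesh under an OnSpawning flag, shakes nearby cameras on non-dedicated instances, and adds an icon message to the local player's HUD.
; The authority binds the STInteractionObject's delegates: CanInteract checks that flag, while OnInteractionEnd is an empty stub.
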(event EventBeginPlay
  (bind _returnvalue (Game|GetPlayerController 0))
  (bind _returnvalue_2 (Transformation|GetActorLocation))
  (|CallParentFunction)
  (Utilities|FlowControl|Sequence
    (:then_0
      (Variables|Default|SetOnSpawning true)
      (Components|MoveComponentTo (Variables|Default|GetStaticMesh) "0, 0, 0" "0, 0, 0" false false 5.0 false)
      (Variables|Default|SetOnSpawning false))
    (:then_1
      (Networking|SwitchHasAuthority
        (:Authority
          (|SetBy-RefVar (Utilities|Array|Get(acopy) (Variables|/Script/ProjectST.STInteractionObjectComponent|GetInteractionDelegates (Variables|Default|GetSTInteractionObject))) (Utilities|Struct|MakeInteractionDelegateSets (EventDispatchers|CreateEvent :!event CanInteract) "(null).None" "(null).None" "(null).None" (EventDispatchers|CreateEvent :!event OnInteractioNEnd))))))
    (:then_2
      (if (not (Networking|IsDedicatedServer))
        (Camera|PlayWorldCameraShake "/Game/ExternalResource/Dragon_Rise/Renders/BP_CamerShake_ReturnStoneSpawn.BP_CamerShake_ReturnStoneSpawn_C" (Transformation|GetActorLocation) 0.0 3e+03 1.0 true)))
    (:then_3
      (if (and (Pawn|IsLocalController _returnvalue) (Class|Controller|IsPlayerController _returnvalue))
        (Class|IBPSTHUDInterface|AddIconInterface(Message) (HUD|GetHUD _returnvalue) "/Engine/Tutorial/Mobile/TutorialAssets/android_Icon.android_Icon" "(X=25.000000,Y=25.000000)" "(R=1.000000,G=1.000000,B=1.000000,A=1.000000)" self "None" (Math|Vector2D|MakeVector2D (.x _returnvalue_2) (.y _returnvalue_2)))))))

(event Collision|EventActorBeginOverlap
  (params (OtherActor :type Actor%20Object%20Reference))
  (|CallParentFunction OtherActor) ; 지금 이 노드는 비활성 상태입니다. \n핀을 끌어서 다른 노드를 연결하면 활성화됩니다.
)

(event EventTick
  (params (DeltaSeconds :type Float%20%28single-precision%29))
  (|CallParentFunction DeltaSeconds) ; 지금 이 노드는 비활성 상태입니다. \n핀을 끌어서 다른 노드를 연결하면 활성화됩니다.
)

(fn ConstructionScript
  (|CallParentFunction))

(fn CanInteract
  (params (Interactor :type Actor%20Object%20Reference) (InteractionInfo :type Interaction%20Info%20Structure%20%28by%20ref%29))
  (return (not (Variables|Default|GetOnSpawning))))

(fn OnInteractionEnd
  (params (Interactor :type Actor%20Object%20Reference) (bIsSuccess :type Boolean) (InteractionInfo :type Interaction%20Info%20Structure%20%28by%20ref%29))
  (return))