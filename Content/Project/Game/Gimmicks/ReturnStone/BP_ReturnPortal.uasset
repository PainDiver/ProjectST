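; BP_ReturnPortal is a single-use return portal that lets the first living player to touch it escape.
; The server binds the capsule overlap, ignores dead characters, then adds an immortal buff state message and activates the BP_STGA_Escape gameplay ability on that player.
; It then marks itself used, turns off its particles through an overlap event that appears to be multicast, and destroys itself after a short delay.
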(event Custom|OnComponentBeginOverlap_이벤트
  (params (OverlappedComponent :type Primitive%20Component%20Object%20Reference) (OtherActor :type Actor%20Object%20Reference) (OtherComp :type Primitive%20Component%20Object%20Reference) (OtherBodyIndex :type Integer) (bFromSweep :type Boolean) (SweepResult :type Hit%20Result%20Structure%20%28by%20ref%29))
  (if (not (Variables|Default|GetIsPortalUsed))
    (bind _asstplayer_character (Utilities|Casting|CastToSTPlayerCharacter OtherActor))
    (bind _returnvalue (Class|STStateInterface|HasState(Message) _asstplayer_character (GameplayTags|MakeLiteralGameplayTag "(TagName=\"State.Dead\")")))
    (if (not _returnvalue)
      (Class|STStateInterface|AddStateReplication(Message) _asstplayer_character (GameplayTags|MakeLiteralGameplayTag "(TagName=\"GE.Buff.Immortal\")"))
      (Abilities|TryActivateAbilitybyClass (Ability|GetAbilitySystemComponent OtherActor) "/Game/Project/GAS/Action/BP_STGA_Escape.BP_STGA_Escape_C" true)
      (Variables|Default|SetIsPortalUsed true)
      (CallFunction|OnOverlapMulti)
      (Utilities|FlowControl|Delay 5.0)
      (Actor|DestroyActor))))

(event Custom|OnOverlap_Multi
  (Components|Activation|Deactivate (Variables|Default|GetParticleSystem)))

(event EventBeginPlay
  (Networking|SwitchHasAuthority
    (:Authority
      (Collision|AssignOnComponentBeginOverlap (Variables|Default|GetCapsule) (delegate Custom|OnComponentBeginOverlap_이벤트)))))

(event Collision|EventActorBeginOverlap
  (params (OtherActor :type Actor%20Object%20Reference)))

(event EventTick
  (params (DeltaSeconds :type Float%20%28single-precision%29)))

(fn ConstructionScript)