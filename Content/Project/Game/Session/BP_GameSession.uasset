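; Game session Blueprint that spawns player characters at random PlayerStarts and sets up their initial gameplay state.
; SpawnPlayer uses fixed row 1 of the character DataTable, ignoring AccountData, and registers the new character for readiness.
; A fire-once STEventManager CharacterPrepared event carries the character and its data in a payload object.
; When it fires, the session grants and activates initial GAS abilities, applies initial effects, then initializes the PlayerState's inventory.
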(event Custom|Register_OnCharacterPrepared
  (params (CharacterData :type Character%20Data%20Structure) (Character :type Pawn%20Object%20Reference))
  (bind _returnvalue (Game|ConstructObjectfromClass Character "/Game/Project/Game/Session/SessionEvent/BP_SessionEvent_OnPlayerStateReady_Object.BP_SessionEvent_OnPlayerStateReady_Object_C" CharacterData Character))
  (Class|STEventManager|RegisterEventSubject (Subsystems|GetSTEventManager) Character "(TagName=\"Event.CharacterPrepared\")" (delegate Custom|OnCharacterPrepared) _returnvalue true))

(event Custom|OnCharacterPrepared
  (params (Data :type Object%20Object%20Reference))
  (bind _asbp_session_event_on_player_state_ready_object (Utilities|Casting|CastToBP_SessionEvent_OnPlayerStateReady_Object Data))
  (CallFunction|StartInitialAction (Variables|/Game/Project/Game/Session/SessionEvent/BP_SessionEvent_OnPlayerStateReady_Object.BP_SessionEvent_OnPlayerStateReady_Object_C|GetCharacterData _asbp_session_event_on_player_state_ready_object) (Variables|/Game/Project/Game/Session/SessionEvent/BP_SessionEvent_OnPlayerStateReady_Object.BP_SessionEvent_OnPlayerStateReady_Object_C|GetCharacter _asbp_session_event_on_player_state_ready_object))
  (bind _asbp_stplayer_state (Utilities|Casting|CastToBP_STPlayerState (Variables|/Script/Engine.Pawn|GetPlayerState (Variables|/Game/Project/Game/Session/SessionEvent/BP_SessionEvent_OnPlayerStateReady_Object.BP_SessionEvent_OnPlayerStateReady_Object_C|GetCharacter _asbp_session_event_on_player_state_ready_object))))
  (Default|InitializeInventoryMulti _asbp_stplayer_state))

(event EventBeginPlay
  (|CallParentFunction)
  (bind _outactors (Actor|GetAllActorsOfClass "/Script/Engine.PlayerStart"))
  (Variables|Default|SetPlayerStarts _outactors))

(event EventTick
  (params (DeltaSeconds :type Float%20%28single-precision%29)))

(fn ConstructionScript)

(fn SpawnPlayer
  (params (PlayerController :type Player%20Controller%20Object%20Reference) (AccountData :type Account%20Data%20Structure%20%28by%20ref%29))
  (bind _playerstarts (Variables|Default|GetPlayerStarts))
  (bind (_outitem _outindex) (Utilities|Array|Random _playerstarts))
  (bind _returnvalue (Utilities|GetDataTableRow "/Game/Project/TableData/CharacterDataTable.CharacterDataTable" (Utilities|String|StringToName (Utilities|String|ToString(Integer) 1)))
    (:then
      (LocalVariables|SetLocalCharacterData _returnvalue)
      (bind _output_get (LocalVariables|SetLocalChosenIndex _outindex))
      (LocalVariables|SetLocalChosenStart _outitem)
      (if (!= _output_get -1)
        (bind _returnvalue_2 (Game|SpawnActorfromClass (.Class (Utilities|Struct|BreakCharacterData (LocalVariables|GetLocalCharacterData))) (Transformation|GetActorTransform (LocalVariables|GetLocalChosenStart)) "AdjustIfPossibleButAlwaysSpawn" "MultiplyWithRoot" PlayerController (Game|GetInstigator (Game|GetGameMode))))
        (CallFunction|RegisteronCharacterPrepared (LocalVariables|GetLocalCharacterData) _returnvalue_2)
        (return (Transformation|GetActorTransform (LocalVariables|GetLocalChosenStart)) _returnvalue_2)))))

(fn StartInitialAction
  (params (CharacterData :type Character%20Data%20Structure) (Character :type Pawn%20Object%20Reference))
  (bind (_initialabilitytostart _initialeffecttostart) (Utilities|Struct|BreakCharacterData CharacterData))
  (bind _returnvalue (Ability|GetAbilitySystemComponent Character))
  (Utilities|FlowControl|Sequence
    (:then_0
      (for _array_element _initialabilitytostart
        (if (Utilities|IsValidClass _array_element)
          (Class|AbilitySystemComponent|GiveAbilityandActivateOnce (Ability|GetAbilitySystemComponent Character) _array_element 0 -1))))
    (:then_1
      (for _array_element_2 _initialeffecttostart
        (if (Utilities|IsValidClass _array_element_2)
          (Utilities|IsValid _returnvalue
            (:Is%20Valid
              (GameplayEffects|ApplyGameplayEffectSpecToSelf _returnvalue (GameplayEffects|MakeOutgoingSpec :self _returnvalue :GameplayEffectClass _array_element_2)))))))))