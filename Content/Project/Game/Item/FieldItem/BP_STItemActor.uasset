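; BP_STItemActor is a field item actor that a character picks up by interacting with it.
; On BeginPlay it hooks an end-interaction event into the first delegate entry of its InteractionObjectComponent.
; When interaction ends, authority checks for success and has STGameState move the item into the interacting character's inventory.
; Remote instances instead spawn a Niagara hit effect at the item's location, regardless of success.
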(event EventBeginPlay
  (|CallParentFunction)
  (CallFunction|BindEvent))

(event Collision|EventActorBeginOverlap
  (params (OtherActor :type Actor%20Object%20Reference)))

(event EventTick
  (params (DeltaSeconds :type Float%20%28single-precision%29)))

(fn ConstructionScript)

(fn BindEvent
  (|SetBy-RefVar (Utilities|Array|Get(acopy) (Variables|/Script/ProjectST.STInteractionObjectComponent|GetInteractionDelegates (Variables|Default|GetInteractionObjectComponent))) (Utilities|Struct|MakeInteractionDelegateSets "(null).None" "(null).None" "(null).None" "(null).None" (EventDispatchers|CreateEvent :!event OnInteractionEnded))))

(fn OnInteractionEnded
  (params (Interactor :type Actor%20Object%20Reference) (bIsSuccess :type Boolean) (InteractionInfo :type Interaction%20Info%20Structure%20%28by%20ref%29))
  (Networking|SwitchHasAuthority
    (:Authority
      (if bIsSuccess
        (bind _asstgame_state (Utilities|Casting|CastToSTGameState (Game|GetGameState)))
        (bind _as캐릭터 (Utilities|Casting|CastToCharacter Interactor))
        (Class|STGameState|MoveFieldItemtoOwner _asstgame_state _as캐릭터 self "INVENTORY")))
    (:Remote
      (Niagara|SpawnSystematLocation "/Game/ExternalResource/MixedVFX/Particles/Projectiles/Hits/NS_LightningArrow_Hit.NS_LightningArrow_Hit" (Transformation|GetActorLocation)))))