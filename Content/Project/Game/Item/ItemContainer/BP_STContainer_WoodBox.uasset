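; Destructible wooden box container with an inventory and a hinged lid that opens on interaction.
; Successful interaction plays a timeline rotating the lid before forwarding to the parent end-interaction logic, and releasing the gimmick closes it.
; STDestruction delegates play wood particles and an impact sound on damage.
; On destruction, mesh and lid are removed; the dedicated server drops all items then destroys the actor, while others add a geometry collection component.
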(event Custom|CloseRid
  (bind _새_트랙_0 (Timeline|CloseRidAnim PlayFromStart)
    (:Update
      (Transformation|SetRelativeRotation (Variables|Default|GetScene) (Math|Rotator|MakeRotator _새_트랙_0 0.0 0.0) false false))))

(event Custom|OpenRid
  (params (Interactor :type Actor%20Object%20Reference) (Res :type Boolean) (Interaction :type Interaction%20Info%20Structure))
  (bind _새_트랙_0 (Timeline|OpenRidAnim PlayFromStart)
    (:Update
      (Transformation|SetRelativeRotation (Variables|Default|GetScene) (Math|Rotator|MakeRotator _새_트랙_0 0.0 0.0) false false))
    (:Finished
      (|CallParentFunction Interactor Res Interaction)
      (Variables|Default|SetIsContainerOpen true))))

(event Custom|OnDestructionDelegate_이벤트
  (Components|DestroyComponent (Variables|Default|GetStaticMesh))
  (if (Networking|IsDedicatedServer)
    (Class|STInventoryComponent|DropAllItem (Variables|Default|GetSTInventory))
    (Utilities|FlowControl|Delay 3.0)
    (Actor|DestroyActor)
    (else
      (AddComponent|AddGeometryCollectionComponent false))))

(event Custom|OnDamageDelegate_이벤트
  (params (Damage :type Integer))
  (bind _staticmesh (Variables|Default|GetStaticMesh))
  (bind _returnvalue (Transformation|GetWorldLocation _staticmesh))
  (Effects|SpawnEmitteratLocation "/Game/ExternalResource/Realistic_Starter_VFX_Pack_Vol2/Particles/Hit/P_Wood.P_Wood" _returnvalue "0, 0, 0" "3.000000,3.000000,3.000000")
  (Audio|PlaySoundatLocation "/Game/ExternalResource/Free_Sounds_Pack/wav/Rock_Impact_11.Rock_Impact_11" _returnvalue "0, 0, 0" 1.0 1.0 0.0 0 0 0 0))

(event EventBeginPlay
  (|CallParentFunction)
  (EventDispatchers|AssignOnDamageDelegate (Variables|Default|GetSTDestruction) (delegate Custom|OnDamageDelegate_이벤트))
  (EventDispatchers|AssignOnDestructionDelegate (Variables|Default|GetSTDestruction) (delegate Custom|OnDestructionDelegate_이벤트)))

(event Collision|EventActorBeginOverlap
  (params (OtherActor :type Actor%20Object%20Reference))
  (|CallParentFunction OtherActor) ; 지금 이 노드는 비활성 상태입니다. \n핀을 끌어서 다른 노드를 연결하면 활성화됩니다.
)

(event EventTick
  (params (DeltaSeconds :type Float%20%28single-precision%29))
  (|CallParentFunction DeltaSeconds) ; 지금 이 노드는 비활성 상태입니다. \n핀을 끌어서 다른 노드를 연결하면 활성화됩니다.
)

(event EventOnInteractorSetGimmick
  (params (Set :type Boolean))
  (|CallParentFunction Set)
  (if (not Set)
    (if (Variables|Default|GetIsContainerOpen)
      (CallFunction|CloseRid))))

(fn ConstructionScript
  (|CallParentFunction))

(fn OnEndInteraction
  (params (Interactor :type Actor%20Object%20Reference) (bIsSuccess :type Boolean) (InteractionInfo :type Interaction%20Info%20Structure%20%28by%20ref%29))
  (if bIsSuccess
    (CallFunction|OpenRid Interactor bIsSuccess InteractionInfo)
    (return)
    (else
      (|CallParentFunction Interactor bIsSuccess InteractionInfo))))