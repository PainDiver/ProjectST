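; Lootable, damageable item container that players investigate to open its inventory, limited to one interactor at a time.
; After a short delay on BeginPlay, the server fills STInventory with fixed items plus percentage rolls from a random bundle DataTable.
; Interaction delegates play an investigation montage and, on success, show the inventory widget to the local player.
; The interactor's gimmick reference drives the busy flag, released on failure or widget close.
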(event EventBeginPlay
  (Utilities|FlowControl|Sequence
    (:then_0
      (CallFunction|BindEvent))
    (:then_1
      (Networking|SwitchHasAuthority
        (:Authority
          (Utilities|FlowControl|Delay 5.0)
          (CallFunction|CreateItems))))))

(event Collision|EventActorBeginOverlap
  (params (OtherActor :type Actor%20Object%20Reference)))

(event EventTick
  (params (DeltaSeconds :type Float%20%28single-precision%29)))

(event EventOnInteractorSetGimmick
  (params (Set :type Boolean))
  (if Set
    (Variables|Default|SetIsOnInteraction true)
    (else
      (Variables|Default|SetIsOnInteraction false))))

(event EventOnGetAttacked
  (params (BreakDamage :type Integer))
  (Class|STDestructionComponent|DamageObject (Variables|Default|GetSTDestruction) BreakDamage))

(fn ConstructionScript
  (|CallParentFunction))

(fn BindEvent
  (|SetBy-RefVar (Utilities|Array|Get(acopy) (Variables|/Script/ProjectST.STInteractionObjectComponent|GetInteractionDelegates (Variables|Default|GetSTInteractionObject))) (Utilities|Struct|MakeInteractionDelegateSets (EventDispatchers|CreateEvent :!event CanInteract) (EventDispatchers|CreateEvent :!event OnStartInteraction) "(null).None" "(null).None" (EventDispatchers|CreateEvent :!event OnEndInteraction))))

(fn CanInteract
  (params (Interactor :type Actor%20Object%20Reference) (InteractionInfo :type Interaction%20Info%20Structure%20%28by%20ref%29))
  (if (Variables|Default|GetIsOnInteraction)
    (return false)
    (else
      (return true))))

(fn OnStartInteraction
  (params (Interactor :type Actor%20Object%20Reference) (InteractionInfo :type Interaction%20Info%20Structure%20%28by%20ref%29))
  (Utilities|FlowControl|Sequence
    (:then_0
      (Networking|SwitchHasAuthority
        (:Authority
          (Class|STInteractionSubjectComponent|SetInteractingGimmick (Actor|GetComponentbyClass Interactor "/Script/ProjectST.STInteractionSubjectComponent") self))))
    (:then_1
      (CallFunction|PlayInteractionAnim Interactor "/Game/Project/Character/Animation/ProcessedAnimation/Interaction/A_Investigation_Montage.A_Investigation_Montage" ""))))

(fn OnEndInteraction
  (params (Interactor :type Actor%20Object%20Reference) (bIsSuccess :type Boolean) (InteractionInfo :type Interaction%20Info%20Structure%20%28by%20ref%29))
  (Utilities|FlowControl|Sequence
    (:then_1
      (if bIsSuccess
        (CallFunction|OpenInventory Interactor)
        (else
          (Networking|SwitchHasAuthority
            (:Authority
              (bind _returnvalue (Class|STCharacterInterface|GetInteractionSubjectComponent(Message) Interactor))
              (Class|STInteractionSubjectComponent|SetInteractingGimmick _returnvalue))))))
    (:then_2
      (CallFunction|PlayInteractionAnim Interactor "/Game/Project/Character/Animation/ProcessedAnimation/Interaction/A_Investigation_Montage.A_Investigation_Montage" "Stop"))))

(fn CreateItems
  (Utilities|FlowControl|Sequence
    (:then_0
      (bind _asstgame_state (Utilities|Casting|CastToSTGameState (Game|GetGameState)))
      (bind _keys (Utilities|Map|Keys (Variables|Default|GetItemsToCreate)))
      (for _array_element _keys
        (bind (_outdata _returnvalue) (Class|STGameState|CreateItemObject _asstgame_state _array_element (.Value (Utilities|Map|Find (Variables|Default|GetItemsToCreate) _array_element))))
        (if _returnvalue
          (Class|STInventoryComponent|AcquireItem (Variables|Default|GetSTInventory) _outdata))))
    (:then_2
      (bind _returnvalue_2 (Utilities|GetDataTableRow "/Game/Project/Game/Item/ItemContainer/RandomItemBundleDataTable.RandomItemBundleDataTable" (Utilities|String|StringToName (Utilities|String|ToString(Integer) (Variables|Default|GetRandomItemBundleData))))
        (:then
          (CallFunction|CreateRandomItems (.RandomItems (Utilities|Struct|BreakRandomItemDataBundle _returnvalue_2))))))))

(fn CreateRandomItems
  (params (Array :type Array%20of%20Random%20Item%20Data%20Structures))
  (bind _asstgame_state (Utilities|Casting|CastToSTGameState (Game|GetGameState)))
  (for _array_element Array
    (if (> (.Percent (Utilities|Struct|BreakRandomItemData _array_element)) (Math|Random|RandomFloatinRange 0.0 1e+02))
      (bind (_outdata _returnvalue) (Class|STGameState|CreateItemObject _asstgame_state (.ID (Utilities|Struct|BreakRandomItemData _array_element)) (.Count (Utilities|Struct|BreakRandomItemData _array_element))))
      (if _returnvalue
        (Class|STInventoryComponent|AcquireItem (Variables|Default|GetSTInventory) _outdata)))))

(fn OpenInventory
  (params (Interactor :type Actor%20Object%20Reference))
  (bind _returnvalue (Game|GetPlayerController 0))
  (bind _as캐릭터 (Utilities|Casting|CastToCharacter Interactor))
  (if (and (Pawn|IsLocallyControlled _as캐릭터) (Pawn|IsPlayerControlled _as캐릭터))
    (bind _returnvalue_2 (Game|ConstructObjectfromClass _returnvalue "/Game/Project/Character/Player/HUD/UIParam/BP_ShowWidget_Status.BP_ShowWidget_Status_C" "NewEnumerator3" (Variables|Default|GetSTInventory) true))
    (EventDispatchers|BindEventtoOnWidgetRemoveDelegate _returnvalue_2 (EventDispatchers|CreateEvent :!event OnInventoryClosed))
    (Class|IBPSTHUDInterface|ShowWidgetbyTagInterface(Message) (HUD|GetHUD _returnvalue) "(TagName=\"UI.StatusBase\")" _returnvalue_2)))

(fn PlayInteractionAnim
  (params (Interactor :type Actor%20Object%20Reference) (AnimMontage :type Anim%20Montage%20Object%20Reference) (StartSectionName :type Name))
  (bind _returnvalue (Class|STStateInterface|GetStates(Message) Interactor))
  (if (not (GameplayTags|HasAnyTags _returnvalue (GameplayTags|MakeLiteralGameplayTagContainer "(GameplayTags=((TagName=\"State.Dead\"),(TagName=\"State.Falling\"),(TagName=\"State.Flying\"),(TagName=\"State.Lying\"),(TagName=\"CombatState.Hit\")))")))
    (bind _asstcharacter_base (Utilities|Casting|CastToSTCharacterBase Interactor))
    (Animation|PlayAnimMontage _asstcharacter_base AnimMontage 1.0 StartSectionName)))

(fn OnInventoryClosed
  (bind _returnvalue (Class|STCharacterInterface|GetInteractionSubjectComponent(Message) (Game|Player|GetPlayerPawn 0)))
  (Class|STInteractionSubjectComponent|RequestSetInteractingGimmickServer _returnvalue))