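; Game instance Blueprint that starts the main-server connection at init and binds packet handlers by net role.
; Clients and standalone games bind login and match packets, storing account data and relaying both results through STEventManager events.
; Dedicated servers bind connection and exit callbacks, to report their command-line batcher ID and port once connected and force-quit when told.
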(event EventPostInitialize
  (CallFunction|BindEvent)
  (Class|STNetManager|StartConnectingtoMainServer (Subsystems|GetSTNetManager)))

(fn BindEvent
  (if (Networking|IsServer)
    (if (Class|KismetSystemLibrary|IsStandalone)
      (EventDispatchers|BindEventtoDeleSCPacketLogin (Class|STNetManager|GetPacketHandler (Subsystems|GetSTNetManager)) (EventDispatchers|CreateEvent :!event SConLogin) :!label _label)
      (EventDispatchers|BindEventtoDeleSCPacketMatch (Class|STNetManager|GetPacketHandler (Subsystems|GetSTNetManager)) (EventDispatchers|CreateEvent :!event SConMatching))
      (else
        (Development|PrintString "BP_STGameInstance_BindEventAsDedicateServer")
        (Utilities|FlowControl|Sequence
          (:then_0
            (EventDispatchers|BindEventtoOnConnected (Subsystems|GetSTNetManager) (EventDispatchers|CreateEvent :!event OnConnected)))
          (:then_1
            (EventDispatchers|BindEventtoDeleSDPacketDediExit (Class|STNetManager|GetPacketHandler (Subsystems|GetSTNetManager)) (EventDispatchers|CreateEvent :!event SDonDediExit))))))
    (else
      (goto _label))))

(fn OnConnected
  (bind _returnvalue (Utilities|GetCommandLine))
  (Class|STNetPacketHandler|SendDataFDSPacketDedi (Class|STNetManager|GetPacketHandler (Subsystems|GetSTNetManager)) (Utilities|Struct|MakeDS_Packet_Dedi (.OutValue (Class|KismetSystemLibrary|ParseParamValue _returnvalue "STBatcherID=")) (.OutValue (Class|KismetSystemLibrary|ParseParamValue _returnvalue "port="))))
  (Development|PrintString (Utilities|String|Append "BTP_STGameInstance) " "Batcher ID" (.OutValue (Class|KismetSystemLibrary|ParseParamValue _returnvalue "STBatcherID=")) "Port " (.OutValue (Class|KismetSystemLibrary|ParseParamValue _returnvalue "port=")))))

(fn SDonDediExit
  (params (Message :type SD%20Packet%20Dedi%20Exit%20Structure%20%28by%20ref%29))
  (Development|PrintString "Dedicate Exit requsted")
  (Class|STGameBlueprintFunctionLibrary|RequestExit true "Dele_SD_Packet_DediExit")
  (return))

(fn SConLogin
  (params (Message :type SC%20Packet%20Login%20Structure%20%28by%20ref%29))
  (bind (_accountinfo _isaccountcreated) (Utilities|Struct|BreakSC_Packet_Login Message))
  (Class|AccountManager|SetLocalAccountData (Subsystems|GetAccountManager) _accountinfo)
  (if _isaccountcreated
    (Development|PrintString "계정 새로 생성됨"))
  (Class|STEventManager|FireEvent (Subsystems|GetSTEventManager) "(TagName=\"Event.Server.Login\")")
  (return))

(fn SConMatching
  (params (Message :type SC%20Packet%20Match%20Structure%20%28by%20ref%29))
  (bind _returnvalue (Game|ConstructObjectfromClass "/Game/Project/Event/BP_Event_MatchData.BP_Event_MatchData_C" Message))
  (Class|STEventManager|FireEvent (Subsystems|GetSTEventManager) "(TagName=\"Event.Server.Match\")" _returnvalue)
  (return))