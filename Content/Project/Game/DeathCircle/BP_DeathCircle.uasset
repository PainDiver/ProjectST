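; Death circle actor, apparently a battle-royale-style zone, that penalizes characters outside its capsule through the Gameplay Ability System.
; TickDamage checks all STCharacterBase actors, applying BP_STGE_DeathCircle outside and removing it inside, with effect handles stored per character but never cleared.
; The server starts a one-second looping timer, presumably for this check.
; Phase logic and shrinking are unfinished: phase handlers are empty and Tick sets the radius to zero.
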(event Custom|SetPhase
  (params (CurrentPhase :type Integer)))

(event EventBeginPlay
  (Networking|SwitchHasAuthority
    (:Authority
      (Utilities|Time|SetTimerbyEvent (EventDispatchers|CreateEvent :!event TickDamage) 1.0 true))))

(event Collision|EventActorBeginOverlap
  (params (OtherActor :type Actor%20Object%20Reference)))

(event EventTick
  (params (DeltaSeconds :type Float%20%28single-precision%29))
  (Components|Capsule|SetCapsuleRadius (Variables|Default|GetCapsule) 0.0 true))

(fn ConstructionScript)

(fn TickDamage
  (if true
    (bind _outactors (Actor|GetAllActorsOfClass "/Script/ProjectST.STCharacterBase"))
    (for _array_element _outactors
      (if (Collision|IsOverlappingActor (Variables|Default|GetCapsule) _array_element :!class /Script/Engine.PrimitiveComponent)
        (if (.ReturnValue (Utilities|Map|Find (Variables|Default|GetPlayersOutOfRange) _array_element))
          (GameplayEffects|RemoveActiveGameplayEffect (Ability|GetAbilitySystemComponent _array_element) (.Value (Utilities|Map|Find (Variables|Default|GetPlayersOutOfRange) _array_element)) -1))
        (elif (.ReturnValue (Utilities|Map|Find (Variables|Default|GetPlayersOutOfRange) _array_element))
          (GameplayEffects|SetActiveGameplayEffectLevel (Ability|GetAbilitySystemComponent _array_element) (.Value (Utilities|Map|Find (Variables|Default|GetPlayersOutOfRange) _array_element)) 0)
          (else
            (bind _returnvalue (GameplayEffects|ApplyGameplayEffectToSelf (Ability|GetAbilitySystemComponent _array_element) "/Game/Project/GAS/Effect/BP_STGE_DeathCircle.BP_STGE_DeathCircle_C" (Math|Conversions|ToFloat(Integer) 0) (GameplayEffects|MakeEffectContext (Ability|GetAbilitySystemComponent _array_element))))
            (Utilities|Map|Add (Variables|Default|GetPlayersOutOfRange) _array_element _returnvalue)))))))

(fn OnRepCurrentPhase
  (if true
    _))