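; BP_GC_Hit is a GameplayCue that plays hit feedback on the struck target: blood splatter, sound and camera shake.
; OnExecute reads the first aggregated source tag (Hit.Head, Hit.Right, Hit.Left) to offset and rotate the emitter attached to the target's mesh, choosing randomly when none matches.
; The camera shakes only when player 0's pawn is the instigator or effect causer, checked in both cue parameters and effect context.
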(event EventBeginPlay)

(event Collision|EventActorBeginOverlap
  (params (OtherActor :type Actor%20Object%20Reference)))

(event EventTick
  (params (DeltaSeconds :type Float%20%28single-precision%29)))

(fn ConstructionScript)

(fn OnExecute
  (params (MyTarget :type Actor%20Object%20Reference) (Parameters :type Gameplay%20Cue%20Parameters%20Structure%20%28by%20ref%29))
  (bind _returnvalue (Game|Player|GetPlayerPawn 0))
  (bind _aggregatedsourcetags (Ability|GameplayCue|BreakGameplayCueParameters Parameters))
  (bind (_normalizedmagnitude _rawmagnitude _effectcontext _matchedtagname _originaltag _aggregatedsourcetags_2 _aggregatedtargettags _location _normal _instigator _effectcauser) (Ability|GameplayCue|BreakGameplayCueParameters Parameters))
  (bind _gameplaytags (GameplayTags|BreakGameplayTagContainer _aggregatedsourcetags))
  (LocalVariables|SetLocalOffsetLoc "0.000000,-0.000000,80.000000")
  (Utilities|FlowControl|Sequence
    (:then_0
      (if (> (Utilities|Array|Length _gameplaytags) 0)
        (|SwitchGameplayTag (Utilities|Array|Get(acopy) _gameplaytags)
          (:Default
            (switch int (Math|Random|RandomIntegerinRange 0 2) :!label _label
              (:0
                (LocalVariables|SetLocalOffsetLoc "0.000000,0.000000,130.000000"))
              (:1
                (LocalVariables|SetLocalOffsetLoc "30.000000,0.000000,80.000000")
                (LocalVariables|SetLocalOffsetRot "30.000000,0.000000,0.000000"))
              (:2
                (LocalVariables|SetLocalOffsetLoc "-30.000000,0.000000,80.000000")
                (LocalVariables|SetLocalOffsetRot "-30.000000,0.000000,0.000000"))))
          (:Hit.Head
            (LocalVariables|SetLocalOffsetLoc "0.000000,0.000000,130.000000"))
          (:Hit.Right
            (LocalVariables|SetLocalOffsetLoc "30.000000,0.000000,80.000000")
            (LocalVariables|SetLocalOffsetRot "30.000000,0.000000,0.000000"))
          (:Hit.Left
            (LocalVariables|SetLocalOffsetLoc "-30.000000,0.000000,80.000000")
            (LocalVariables|SetLocalOffsetRot "-30.000000,0.000000,0.000000")))
        (else
          (goto _label))))
    (:then_1
      (bind _returnvalue_2 (Effects|SpawnEmitterAttached "/Game/ExternalResource/Realistic_Starter_VFX_Pack_Vol2/Particles/Blood/P_Blood_Splat_Cone.P_Blood_Splat_Cone" (Actor|GetComponentbyClass MyTarget "/Script/Engine.MeshComponent") "Root" "0, 0, 0" "0, 0, 0" "1.000000,1.000000,1.000000" "SnapToTargetIncludingScale"))
      (Transformation|AddLocalOffset _returnvalue_2 (LocalVariables|GetLocalOffsetLoc) false true)
      (Transformation|AddRelativeRotation _returnvalue_2 (LocalVariables|GetLocalOffsetRot) false false)
      (Audio|PlaySoundatLocation MyTarget "/Game/Project/Sound/HitSound.HitSound" (Transformation|GetActorLocation MyTarget) "0, 0, 0" 1.0 1.0 0.0 0 0 0 0))
    (:then_2
      (if (or (or (== (Class|AbilitySystemBlueprintLibrary|EffectContextGetInstigatorActor _effectcontext) _returnvalue) (== (Class|AbilitySystemBlueprintLibrary|EffectContextGetEffectCauser _effectcontext) _returnvalue)) (or (== _instigator _returnvalue) (== _effectcauser _returnvalue)))
        (CameraShakes|StartCameraShake (Variables|/Script/Engine.PlayerController|GetPlayerCameraManager (Game|GetPlayerController 0)) "/Game/Project/Character/Player/Camera/BP_CS_Hit.BP_CS_Hit_C" 1.0 "CameraLocal" "0, 0, 0")))
    (:then_3
      (return true))))