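; Katana guard gameplay ability that raises and releases a guard stance with montages based on the input trigger state.
; On activation, the locally controlled side waits for one input gameplay event, reads its trigger state from ComboInputData, and processes it locally and through a server call.
; Triggered or Started plays the guard-start montage, Completed plays the guard-to-idle montage, and Ongoing or Canceled ends the ability.
; Either montage finishing or being interrupted also ends it.
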(event Custom|ProcessGuard
  (params (Selection :type ETriggerEvent%20Enum :default "None"))
  (switch Utilities|FlowControl|Switch|SwitchonETriggerEvent Selection
    (:Triggered
      (|PlayMontageandWaitProxy "Guard" "/Game/Project/Character/Animation/ProcessedAnimation/Guard/ARPG_Samurai_Anim_UE_Guard_B_Start_Montage.ARPG_Samurai_Anim_UE_Guard_B_Start_Montage" 1.0 "None" true 1.0 0.0 false :!label _label
        (:OnCompleted
          _)
        (:OnInterrupted
          _)
        (:OnCancelled
          _))
      (Ability|EndAbility))
    (:Started
      (goto _label))
    (:Ongoing
      (Ability|EndAbility :!label _label_2))
    (:Canceled
      (goto _label_2))
    (:Completed
      (|PlayMontageandWaitProxy "ReleaseGuard" "/Game/Project/Character/Animation/ProcessedAnimation/Guard/ARPG_Samurai_Anim_UE_Guard_B_to_Idle_Montage.ARPG_Samurai_Anim_UE_Guard_B_to_Idle_Montage" 1.0 "None" true 1.0 0.0 false
        (:OnCompleted
          _)
        (:OnInterrupted
          _)
        (:OnCancelled
          _))
      (Ability|EndAbility))))

(event Custom|ProcessGuard_Server
  (params (Selection :type ETriggerEvent%20Enum :default "None"))
  (CallFunction|ProcessGuard Selection))

(event Ability|EventOnEndAbility
  (params (bWasCancelled :type Boolean)))

(event Ability|EventActivateAbility
  (Pawn|IsLocallyControlled
    (:True
      (bind _payload (Ability|Tasks|WaitGameplayEvent "(TagName=\"Input.InputInstance\")" 0 true)
        (:EventReceived
          (bind _ascombo_input_data (Utilities|Casting|CastToComboInputData (Utilities|Struct|BreakGameplayEventData _payload))
            (:then
              (CallFunction|ProcessGuard (Utilities|Struct|BreakInputActionInstance (Variables|/Script/ProjectST.ComboInputData|GetInputInstance _ascombo_input_data)))
              (CallFunction|ProcessGuardServer (Utilities|Struct|BreakInputActionInstance (Variables|/Script/ProjectST.ComboInputData|GetInputInstance _ascombo_input_data))))
            (:CastFailed
              (Ability|EndAbility))))))))