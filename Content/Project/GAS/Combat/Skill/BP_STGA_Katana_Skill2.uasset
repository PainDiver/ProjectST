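; BP_STGA_Katana_Skill2 is a gameplay ability for the katana's second skill, a slash that launches a wave projectile.
; After a successful commit, it plays the Katana_Skill2 montage with reduced root motion and waits for a Skill.KatanaSkill2 gameplay event.
; That event spawns an authority-only BP_STProjectile_KatanaWave at the avatar, facing its forward vector with the pawn as instigator.
; The ability ends when the montage completes, blends out or is interrupted or cancelled, or when the commit fails.
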(event Custom|Slash
  (bind _returnvalue (Ability|GetAvatarActorfromActorInfo))
  (|PlayMontageandWaitProxy "Skill2Anim" "/Game/Project/Character/Animation/ProcessedAnimation/Skill/Katana/Skill2/Katana_Skill2.Katana_Skill2" 1.0 "None" true 0.6 0.0 false
    (:then
      (Ability|Async|WaitGameplayEventToActor (Ability|GetAvatarActorfromActorInfo) "(TagName=\"Skill.KatanaSkill2\")" true
        (:EventReceived
          (bind _as폰 (Utilities|Casting|CastToPawn _returnvalue))
          (|SpawnActor 0 (Transformation|GetActorLocation _returnvalue) (Math|Conversions|RotationFromXVector (Transformation|GetActorForwardVector (Ability|GetAvatarActorfromActorInfo))) "/Game/Project/Game/Projectile/BP_STProjectile_KatanaWave.BP_STProjectile_KatanaWave_C" true _as폰))))
    (:OnCompleted
      (Ability|EndAbility :!label _label))
    (:OnBlendOut
      (goto _label))
    (:OnInterrupted
      (goto _label))
    (:OnCancelled
      (goto _label))))

(event Ability|EventActivateAbility
  (bind _returnvalue (Ability|CommitAbility))
  (if _returnvalue
    (CallFunction|Slash)
    (else
      (Ability|EndAbility))))

(event Ability|EventOnEndAbility
  (params (bWasCancelled :type Boolean)))