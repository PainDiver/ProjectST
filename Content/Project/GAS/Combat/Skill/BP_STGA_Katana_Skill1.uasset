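; Katana Skill 1 gameplay ability: plays a start montage, then one of four phased slashes with motion warping toward a point ahead.
; On the locally controlled side, the first phase gameplay event cancels the other waits and sets a warp point that lies farther forward in later phases.
; SyncNetDataGenericData shares phase and point (server-authored for AI, client-authored otherwise), then Slash plays the matching montage and sets the warp target.
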(event Custom|Slash
  (params (Phase :type Integer) (WarpTarget :type Vector))
  (|PlayMontageandWaitProxy "Skill1Anim" (Utilities|Select :Index Phase :Option%200 0 :Option%201 "/Game/Project/Character/Animation/ProcessedAnimation/Skill/Katana/Skill1/Katana_Skill1_Slash1.Katana_Skill1_Slash1" :Option%202 "/Game/Project/Character/Animation/ProcessedAnimation/Skill/Katana/Skill1/Katana_Skill1_Slash2.Katana_Skill1_Slash2" :Option%203 "/Game/Project/Character/Animation/ProcessedAnimation/Skill/Katana/Skill1/Katana_Skill1_Slash3.Katana_Skill1_Slash3" :Option%204 "/Game/Project/Character/Animation/ProcessedAnimation/Skill/Katana/Skill1/Katana_Skill1_Slash4.Katana_Skill1_Slash4") 1.0 "None" true 1.0 0.0 false
    (:then
      (Class|MotionWarpingComponent|AddorUpdateWarpTargetfromLocationandRotation (Actor|GetComponentbyClass (Ability|GetAvatarActorfromActorInfo) "/Script/ProjectST.STMotionWarpingComponent") "Skill1Warp" WarpTarget (Math|Rotator|FindLookatRotation (Transformation|GetActorLocation (Ability|GetAvatarActorfromActorInfo)) WarpTarget)))
    (:OnCompleted
      (Ability|EndAbility :!label _label))
    (:OnBlendOut
      (goto _label))
    (:OnInterrupted
      (goto _label))
    (:OnCancelled
      (goto _label))))

(event Ability|EventActivateAbility
  (bind _returnvalue (Ability|GetAvatarActorfromActorInfo))
  (bind _returnvalue_2 (Ability|CommitAbility))
  (if _returnvalue_2
    (|PlayMontageandWaitProxy "Skill1Anim" "/Game/Project/Character/Animation/ProcessedAnimation/Skill/Katana/Skill1/Katana_Skill1_Start.Katana_Skill1_Start" 1.0 "None" true 1.0 0.0 false
      (:then
        (Variables|Default|SetIsOnWaiting true)
        (Pawn|IsLocallyControlled
          (:True
            (Utilities|FlowControl|Sequence
              (:then_0
                (bind (_asynctaskproxy _payload) (Ability|Async|WaitGameplayEventToActor (Ability|GetAvatarActorfromActorInfo) "(TagName=\"Skill.KatanaSkill1.Phase1\")" true)
                  (:EventReceived
                    (Variables|Default|SetPayload _payload))))
              (:then_1
                (bind (_asynctaskproxy_2 _payload_2) (Ability|Async|WaitGameplayEventToActor (Ability|GetAvatarActorfromActorInfo) "(TagName=\"Skill.KatanaSkill1.Phase2\")" true)
                  (:EventReceived
                    (Variables|Default|SetPayload _payload_2))))
              (:then_2
                (bind (_asynctaskproxy_3 _payload_3) (Ability|Async|WaitGameplayEventToActor (Ability|GetAvatarActorfromActorInfo) "(TagName=\"Skill.KatanaSkill1.Phase3\")" true)
                  (:EventReceived
                    (Variables|Default|SetPayload _payload_3))))
              (:then_3
                (bind (_asynctaskproxy_4 _payload_4) (Ability|Async|WaitGameplayEventToActor (Ability|GetAvatarActorfromActorInfo) "(TagName=\"Skill.KatanaSkill1.Phase4\")" true)
                  (:EventReceived
                    (Variables|Default|SetPayload _payload_4)))))
            (Ability|Async|EndAction _asynctaskproxy_2)
            (Variables|Default|SetIsOnWaiting false)
            (bind _asans_event_skill_1 (Utilities|Casting|CastToANS_Event_Skill1 (Utilities|Struct|BreakGameplayEventData (Variables|Default|GetPayload))))
            (bind _data (|SyncNetDataGenericData (select (Utilities|IsValid (AI|GetAIController (Ability|GetAvatarActorfromActorInfo))) "ServerGiveData" "ClientGiveData") (Utilities|Struct|MakeSTGenericGameplayAbilityTargetDataParams (Utilities|Array|MakeArray (+ (Transformation|GetActorLocation _returnvalue) (* (Transformation|GetActorForwardVector _returnvalue) (Utilities|Select :Index (Variables|/Game/Project/Character/Animation/NotifyEvent/AnimNotifyState/Event/ANS_Event_Skill1.ANS_Event_Skill1_C|GetPhase _asans_event_skill_1) :Option%200 0.0 :Option%201 3.5e+02 :Option%202 5e+02 :Option%203 6e+02 :Option%204 7e+02)))) (Utilities|Array|MakeArray (Variables|/Game/Project/Character/Animation/NotifyEvent/AnimNotifyState/Event/ANS_Event_Skill1.ANS_Event_Skill1_C|GetPhase _asans_event_skill_1))))
              (:OnSync
                (CallFunction|Slash (Utilities|Array|Get(acopy) (.Ints (Utilities|Struct|BreakSTGenericGameplayAbilityTargetDataParams _data))) (Utilities|Array|Get(acopy) (.Vectors (Utilities|Struct|BreakSTGenericGameplayAbilityTargetDataParams _data)))))))
          (:False
            (bind _data_2 (|SyncNetDataGenericData (select (Utilities|IsValid (AI|GetAIController (Ability|GetAvatarActorfromActorInfo))) "ServerGiveData" "ClientGiveData"))
              (:OnSync
                (CallFunction|Slash (Utilities|Array|Get(acopy) (.Ints (Utilities|Struct|BreakSTGenericGameplayAbilityTargetDataParams _data_2))) (Utilities|Array|Get(acopy) (.Vectors (Utilities|Struct|BreakSTGenericGameplayAbilityTargetDataParams _data_2)))))))))
      (:OnCompleted
        (Pawn|IsLocallyControlled :!label _label
          (:True
            (if (Variables|Default|GetIsOnWaiting)
              (Ability|EndAbility)))))
      (:OnBlendOut
        (goto _label))
      (:OnInterrupted
        (goto _label))
      (:OnCancelled
        (goto _label)))
    (else
      (Ability|EndAbility))))

(event Ability|EventOnEndAbility
  (params (bWasCancelled :type Boolean)))