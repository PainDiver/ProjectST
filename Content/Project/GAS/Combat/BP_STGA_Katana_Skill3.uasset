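; Gameplay ability for the katana's third skill, a slash driven by a montage.
; On activation it commits, then plays Katana_Skill3 with scaled-down root motion, ending when the montage completes, blends out or is stopped, or if commit fails.
; Slash_Server also triggers the slash but is not called here.
; An unconnected branch that waits for a KatanaSkill2 event to spawn a wave projectile never runs.
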(event Custom|Slash_Server
  (CallFunction|Slash))

(event Custom|Slash
  (|PlayMontageandWaitProxy "Skill3Anim" "/Game/Project/Character/Animation/ProcessedAnimation/Skill/Katana/Skill3/Katana_Skill3.Katana_Skill3" 1.0 "None" true 0.6 0.0 false
    (:OnCompleted
      _)
    (:OnBlendOut
      _)
    (:OnInterrupted
      _)
    (:OnCancelled
      _))
  (Ability|EndAbility))

(event Ability|EventActivateAbility
  (bind _returnvalue (Ability|CommitAbility))
  (if _returnvalue
    (CallFunction|Slash)
    (else
      (Ability|EndAbility))))

(event Ability|EventOnEndAbility
  (params (bWasCancelled :type Boolean)))