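; Katana parry gameplay ability that turns the avatar toward the instigator and plays a parry montage.
; On authority it waits once for the GA.Action.Parry event and reads the perfect-parry flag from its hit-info payload.
; It runs the parry directly and through a ProcessParry server wrapper.
; A perfect parry speeds up the montage and chains a random heavy-attack counter before ending; a normal parry just ends.
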(event Custom|ProcessParry
  (params (Target :type Actor%20Object%20Reference) (IsPerfectParry :type Boolean))
  (Transformation|SetActorRotation (Ability|GetAvatarActorfromActorInfo) (Math|Rotator|MakeRotator 0.0 0.0 (.yaw (Math|Rotator|FindLookatRotation (Transformation|GetActorLocation (Ability|GetAvatarActorfromActorInfo)) (Transformation|GetActorLocation Target)))))
  (|PlayMontageandWaitProxy "Parry" "/Game/Project/Character/Animation/ProcessedAnimation/Parry/ARPG_Samurai_Anim_UE_Parry_Montage.ARPG_Samurai_Anim_UE_Parry_Montage" (select IsPerfectParry 3.0 1.0) "None" true 1.0 0.0 false
    (:OnCompleted
      _)
    (:OnBlendOut
      _)
    (:OnInterrupted
      _)
    (:OnCancelled
      _))
  (if IsPerfectParry
    (|PlayMontageandWaitProxy "ParryAttack" (.OutItem (Utilities|Array|Random (Utilities|Array|MakeArray "/Game/Project/Character/Animation/ProcessedAnimation/Parry/ARPG_Samurai_Anim_UE_Attack_Heavy2_Montage.ARPG_Samurai_Anim_UE_Attack_Heavy2_Montage" "/Game/Project/Character/Animation/ProcessedAnimation/Parry/ARPG_Samurai_Anim_UE_Attack_HeavyB_Montage.ARPG_Samurai_Anim_UE_Attack_HeavyB_Montage"))) 1.0 "None" true 1.0 0.0 false
      (:OnCompleted
        _)
      (:OnInterrupted
        _)
      (:OnCancelled
        _))
    (Ability|EndAbility)
    (else
      (Ability|EndAbility))))

(event Custom|ProcessParry_Server
  (params (Target :type Actor%20Object%20Reference) (IsPerfectParry :type Boolean))
  (CallFunction|ProcessParry Target IsPerfectParry))

(event Ability|EventOnEndAbility
  (params (bWasCancelled :type Boolean)))

(event Ability|EventActivateAbility
  (Ability|HasAuthority
    (:True
      (bind _payload (Ability|Tasks|WaitGameplayEvent "(TagName=\"GA.Action.Parry\")" 0 true)
        (:EventReceived
          (bind _asbp_hit_info_object (Utilities|Casting|CastToBP_HitInfoObject (.OptionalObject (Utilities|Struct|BreakGameplayEventData _payload))))
          (CallFunction|ProcessParry (.Instigator (Utilities|Struct|BreakGameplayEventData _payload)) (Variables|/Game/Project/GAS/Action/BP_HitInfoObject.BP_HitInfoObject_C|GetIsPerfectParry _asbp_hit_info_object))
          (CallFunction|ProcessParryServer (.Instigator (Utilities|Struct|BreakGameplayEventData _payload)) (Variables|/Game/Project/GAS/Action/BP_HitInfoObject.BP_HitInfoObject_C|GetIsPerfectParry _asbp_hit_info_object)))))))