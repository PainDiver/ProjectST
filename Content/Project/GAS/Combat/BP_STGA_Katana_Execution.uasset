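; Katana execution gameplay ability that plays an execution montage on the avatar.
; On activation it waits once for a GA.Execution gameplay event, using the truncated event magnitude as the row name into the execution info data table.
; The row's montage plays directly and is also passed to a client execute event that plays it too.
; The ability ends when the montage completes, is interrupted or cancelled, or when no row is found.
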(event Custom|Execute_Client
  (params (Anim :type Anim%20Montage%20Object%20Reference))
  (|PlayMontageandWaitProxy "ExecutionAnim" Anim 1.0 "None" true 1.0 0.0 false
    (:OnCompleted
      _)
    (:OnInterrupted
      _)
    (:OnCancelled
      _))
  (Ability|EndAbility))

(event Ability|EventActivateAbility
  (bind _payload (Ability|Async|WaitGameplayEventToActor (Ability|GetAvatarActorfromActorInfo) "(TagName=\"GA.Execution\")" true)
    (:EventReceived
      (bind _returnvalue (Utilities|GetDataTableRow "/Game/Project/TableData/ExecutionInfoTable.ExecutionInfoTable" (Utilities|String|StringToName (Utilities|String|ToString(Integer) (Math|Float|Truncate (.EventMagnitude (Utilities|Struct|BreakGameplayEventData _payload))))))
        (:then
          (CallFunction|ExecuteClient (Utilities|Struct|BreakExecutionInfo _returnvalue))
          (|PlayMontageandWaitProxy "ExecutionAnim" (Utilities|Struct|BreakExecutionInfo _returnvalue) 1.0 "None" true 1.0 0.0 false
            (:OnCompleted
              _)
            (:OnInterrupted
              _)
            (:OnCancelled
              _))
          (Ability|EndAbility))
        (:RowNotFound
          (Ability|EndAbility))))))

(event Ability|EventOnEndAbility
  (params (bWasCancelled :type Boolean)))