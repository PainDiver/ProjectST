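; Gameplay ability for a samurai sway: a directional evade, or a dodge when there is no input.
; The locally controlled client converts last movement input into a normalized actor-space direction and sends it through SyncNetDataVector (ClientGiveData).
; On sync, PickSway thresholds that direction into an evade montage, with pure right reusing the forward-right one.
; The ability plays the montage and ends on blend out, interruption or cancel.
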(event Ability|EventActivateAbility
  (Pawn|IsLocallyControlled
    (:True
      (bind _as캐릭터 (Utilities|Casting|CastToCharacter (Ability|GetAvatarActorfromActorInfo)))
      (Variables|Default|SetInputDir (Class|KismetMathLibrary|VectorNormal2D (Math|Transform|InverseTransformDirection (Transformation|GetActorTransform _as캐릭터) (Pawn|Components|PawnMovement|GetLastInputVector (Variables|/Script/Engine.Character|GetCharacterMovement _as캐릭터))) 0.0001)))
    (:False
      (Variables|Default|SetInputDir "0, 0, 0")))
  (bind _vector (|SyncNetDataVector "ClientGiveData" (Utilities|Array|MakeArray (Variables|Default|GetInputDir)))
    (:OnSync
      (bind _pickedsway (CallFunction|PickSway (Utilities|Array|Get(acopy) _vector)))
      (|PlayMontageandWaitProxy "Sway" _pickedsway 1.0 "None" true 1.0 0.0 false
        (:OnBlendOut
          _)
        (:OnInterrupted
          _)
        (:OnCancelled
          _))
      (Ability|EndAbility))))

(event Ability|EventOnEndAbility
  (params (bWasCancelled :type Boolean)))

(fn PickSway
  (params (Input :type Vector))
  (bind (_x _y) (Math|Vector|BreakVector Input))
  (Utilities|FlowControl|Sequence
    (:then_0
      (if (> _x 0.5)
        (LocalVariables|SetIsForward true)
        (elif (< _x -0.5)
          (LocalVariables|SetIsBackward true))))
    (:then_1
      (if (> _y 0.5)
        (LocalVariables|SetIsRight true)
        (elif (< _y -0.5)
          (LocalVariables|SetIsLeft true))))
    (:then_2
      (if (LocalVariables|GetIsForward)
        (if (LocalVariables|GetIsRight)
          ;[0.15 0.15 0.15 0.5] FR
          (return "/Game/Project/Character/Animation/ProcessedAnimation/Evade/ARPG_Samurai_Anim_UE_Evade_Forward_Right_Montage.ARPG_Samurai_Anim_UE_Evade_Forward_Right_Montage")
          (elif (LocalVariables|GetIsLeft)
            ;[0.15 0.15 0.15 0.5] FL
            (return "/Game/Project/Character/Animation/ProcessedAnimation/Evade/ARPG_Samurai_Anim_UE_Evade_Forward_Left_Montage.ARPG_Samurai_Anim_UE_Evade_Forward_Left_Montage")
            (else
              ;[0.15 0.15 0.15 0.5] F
              (return "/Game/Project/Character/Animation/ProcessedAnimation/Evade/ARPG_Samurai_Anim_UE_Evade_Forward_Montage.ARPG_Samurai_Anim_UE_Evade_Forward_Montage"))))
        (elif (LocalVariables|GetIsBackward)
          (if (LocalVariables|GetIsRight)
            ;[0.15 0.15 0.15 0.5] BR
            (return "/Game/Project/Character/Animation/ProcessedAnimation/Evade/ARPG_Samurai_Anim_UE_Evade_Backward_Right_Montage.ARPG_Samurai_Anim_UE_Evade_Backward_Right_Montage")
            (elif (LocalVariables|GetIsLeft)
              ;[0.15 0.15 0.15 0.5] BL
              (return "/Game/Project/Character/Animation/ProcessedAnimation/Evade/ARPG_Samurai_Anim_UE_Evade_Backward_Left_Montage.ARPG_Samurai_Anim_UE_Evade_Backward_Left_Montage")
              (else
                ;[0.15 0.15 0.15 0.5] B
                (return "/Game/Project/Character/Animation/ProcessedAnimation/Evade/ARPG_Samurai_Anim_UE_Evade_Backward_Montage.ARPG_Samurai_Anim_UE_Evade_Backward_Montage"))))
          (elif (LocalVariables|GetIsRight)
            ;[0.15 0.15 0.15 0.5] R
            (return "/Game/Project/Character/Animation/ProcessedAnimation/Evade/ARPG_Samurai_Anim_UE_Evade_Forward_Right_Montage.ARPG_Samurai_Anim_UE_Evade_Forward_Right_Montage")
            (elif (LocalVariables|GetIsLeft)
              ;[0.15 0.15 0.15 0.5] L
              (return "/Game/Project/Character/Animation/ProcessedAnimation/Evade/ARPG_Samurai_Anim_UE_Evade_Left_Montage.ARPG_Samurai_Anim_UE_Evade_Left_Montage")
              (else
                ;[0.15 0.15 0.15 0.5] Nothing -> Dodge
                (return "/Game/Project/Character/Animation/ProcessedAnimation/Evade/ARPG_Samurai_Anim_UE_Dodge_Montage.ARPG_Samurai_Anim_UE_Dodge_Montage")))))))))