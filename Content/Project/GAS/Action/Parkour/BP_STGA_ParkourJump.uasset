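; Gameplay ability that performs a parkour jump on the avatar Character by playing the Parkour_ParkourJump montage.
; On activation it maps forward velocity in actor space to a clamped root motion translation scale, so slower movement gives a shorter jump.
; A SyncNetData task passes that scale as client-given target data before the montage plays with it.
; The ability ends when the montage completes, blends out, is interrupted or is cancelled.
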(event Ability|EventActivateAbility
  (bind _returnvalue (Ability|GetAvatarActorfromActorInfo))
  (bind _as캐릭터 (Utilities|Casting|CastToCharacter _returnvalue))
  (bind _data (|SyncNetDataGenericData "ClientGiveData" (Utilities|Struct|MakeSTGenericGameplayAbilityTargetDataParams (Utilities|Array|MakeArray (Math|Float|MapRangeClamped (.X (Math|Vector|BreakVector (Math|Vector|UnrotateVector (Transformation|GetVelocity _returnvalue) (Transformation|GetActorRotation _as캐릭터)))) 0.0 7e+02 0.4 1.0))))
    (:OnSync
      (|PlayMontageandWaitProxy "ParkourJump" "/Game/Project/Character/Animation/ProcessedAnimation/Parkour/JumpLanding/Parkour_ParkourJump.Parkour_ParkourJump" 1.0 "None" true (Utilities|Array|Get(acopy) (.Floats (Utilities|Struct|BreakSTGenericGameplayAbilityTargetDataParams _data))) 0.0 false
        (:OnCompleted
          _)
        (:OnBlendOut
          _)
        (:OnInterrupted
          _)
        (:OnCancelled
          _))
      (Ability|EndAbility))))

(event Ability|EventOnEndAbility
  (params (bWasCancelled :type Boolean)))