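; Gameplay ability that performs a parkour vault on the avatar character.
; The locally controlled client waits for a Parkour.Vault event, packs its montage, ignored walls and parkour points into generic target data and syncs it client-to-server.
; Vault then makes the capsule ignore those walls, sets indexed VaultWarp motion warp targets facing the first vector, and plays the montage.
; When the montage ends, it restores collision, clears parkour progress and ends.
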(event Custom|Vault
  (params (STGenericGameplayAbilityTargetDataParams :type ST%20Generic%20Gameplay%20Ability%20Target%20Data%20Params%20Structure%20%28by%20ref%29))
  (bind (_objects _vectors) (Utilities|Struct|BreakSTGenericGameplayAbilityTargetDataParams STGenericGameplayAbilityTargetDataParams))
  (bind _as캐릭터 (Utilities|Casting|CastToCharacter (Ability|GetAvatarActorfromActorInfo)))
  (Utilities|FlowControl|Sequence
    (:then_1
      (for _array_element _objects
        (bind _as프리미티브_컴포넌트 (Utilities|Casting|CastToPrimitiveComponent _array_element))
        (Class|PrimitiveComponent|IgnoreComponentwhenMoving (Variables|/Script/Engine.Character|GetCapsuleComponent _as캐릭터) _as프리미티브_컴포넌트 true)))
    (:then_2
      (for _index (range 1 (- (Utilities|Array|Length _vectors) 1))
        (Class|MotionWarpingComponent|AddorUpdateWarpTargetfromLocationandRotation (Actor|GetComponentbyClass (Ability|GetAvatarActorfromActorInfo) "/Script/ProjectST.STMotionWarpingComponent") (Utilities|String|StringToName (Utilities|String|Append (Utilities|String|MakeLiteralString "VaultWarp") (Utilities|String|ToString(Integer) (- _index 1)))) (Utilities|Array|Get(acopy) _vectors _index) (Math|Conversions|RotationFromXVector (Utilities|Array|Get(acopy) _vectors)))))
    (:then_3
      (bind _as애님_몽타주 (Utilities|Casting|CastToAnimMontage (Utilities|Array|Get(acopy) _objects)))
      (|PlayMontageandWaitProxy "Vault" _as애님_몽타주 1.0 "None" true 1.0 0.0 false
        (:OnCompleted
          _)
        (:OnBlendOut
          _)
        (:OnInterrupted
          _)
        (:OnCancelled
          _))
      (Class|PrimitiveComponent|ClearMoveIgnoreComponents (Variables|/Script/Engine.Character|GetCapsuleComponent _as캐릭터))
      (Class|STParkourComponent|SetParkourProgress (Actor|GetComponentbyClass (Ability|GetAvatarActorfromActorInfo) "/Script/ProjectST.STParkourComponent") false)
      (Ability|EndAbility))))

(event Ability|EventActivateAbility
  (bind _objects (Variables|Default|GetObjects))
  (Pawn|IsLocallyControlled
    (:True
      (bind _payload (Ability|Async|WaitGameplayEventToActor (Ability|GetAvatarActorfromActorInfo) "(TagName=\"Parkour.Vault\")" true)
        (:EventReceived
          (Utilities|Array|Clear (Variables|Default|GetObjects))
          (bind _asbp_parkour_data (Utilities|Casting|CastToBP_ParkourData (Utilities|Struct|BreakGameplayEventData _payload)))
          (Utilities|Array|Add _objects (Variables|/Game/Project/Character/Player/Parkour/BP_ParkourData.BP_ParkourData_C|GetMontage _asbp_parkour_data))
          (Utilities|Array|AppendArray _objects (Variables|/Game/Project/Character/Player/Parkour/BP_ParkourData.BP_ParkourData_C|GetIgnoredWalls _asbp_parkour_data))
          (bind _data (|SyncNetDataGenericData "ClientGiveData" (Utilities|Struct|MakeSTGenericGameplayAbilityTargetDataParams (Variables|Default|GetObjects) (Variables|/Game/Project/Character/Player/Parkour/BP_ParkourData.BP_ParkourData_C|GetParkourPoints _asbp_parkour_data)))
            (:OnSync
              (CallFunction|Vault _data))))))
    (:False
      (bind _data_2 (|SyncNetDataGenericData "ClientGiveData" (Utilities|Struct|MakeSTGenericGameplayAbilityTargetDataParams))
        (:OnSync
          (CallFunction|Vault _data_2))))))