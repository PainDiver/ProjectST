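; Gameplay ability that handles a character's death.
; The server waits for a GA.Action.Dead event, replicates State.Dead and sends the payload's montage to the client through a net data sync, so both sides play it.
; When the montage finishes or is interrupted, State.Dead is sent again and the ability ends.
; On end, the server gives away the victim's inventory, while the owning client fades the HUD and opens the login map on a timer.
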(event Custom|PlayDeadAnim
  (params (MontageToPlay :type Anim%20Montage%20Object%20Reference))
  (|PlayMontageandWaitProxy "Dead" MontageToPlay 1.0 "None" false 1.0 0.0 false
    (:OnCompleted
      _)
    (:OnBlendOut
      _)
    (:OnInterrupted
      _)
    (:OnCancelled
      _))
  (Class|STStateInterface|AddStateReplication(Message) (Ability|GetAvatarActorfromActorInfo) (GameplayTags|MakeLiteralGameplayTag "(TagName=\"State.Dead\")"))
  (Ability|EndAbility))

(event Ability|EventActivateAbility
  (Ability|HasAuthority
    (:True
      (bind _payload (Ability|Async|WaitGameplayEventToActor (Ability|GetAvatarActorfromActorInfo) "(TagName=\"GA.Action.Dead\")" true)
        (:EventReceived
          (Class|STStateInterface|AddStateReplication(Message) (Ability|GetAvatarActorfromActorInfo) (GameplayTags|MakeLiteralGameplayTag "(TagName=\"State.Dead\")")))))
    (:False
      _))
  (bind _data (|SyncNetDataGenericData "ServerGiveData" (Utilities|Struct|MakeSTGenericGameplayAbilityTargetDataParams (Utilities|Array|MakeArray (Utilities|Struct|BreakGameplayEventData _payload))))
    (:OnSync
      (bind _as애님_몽타주 (Utilities|Casting|CastToAnimMontage (Utilities|Array|Get(acopy) (.Objects (Utilities|Struct|BreakSTGenericGameplayAbilityTargetDataParams _data))))
        (:then
          (CallFunction|PlayDeadAnim _as애님_몽타주))
        (:CastFailed
          (Ability|EndAbility))))))

(event Ability|EventOnEndAbility
  (params (bWasCancelled :type Boolean))
  (|CallParentFunction bWasCancelled)
  (Ability|HasAuthority
    (:True
      (Class|IBPSTGameState|GiveAwayInventoryInterface(Message) (Game|GetGameState) (Ability|GetAvatarActorfromActorInfo) false))
    (:False
      (Pawn|IsLocallyControlled
        (:True
          (Class|IBPSTHUDInterface|FadeinOutInterface(Message) (HUD|GetHUD (Game|GetPlayerController 0)) true 3.0 false)
          (Class|IBPSTGameInstance|OpenLevelbyTagInterface(Message) (Game|GetGameInstance) "(TagName=\"Level.LoginMap\")" true "" 5.0))))))