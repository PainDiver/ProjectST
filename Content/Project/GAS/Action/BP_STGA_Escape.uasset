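; BP_STGA_Escape is a Gameplay Ability that makes the avatar actor vanish in an escape effect.
; On activation it sets the avatar's CustomTimeDilation to zero, hides all its skeletal meshes and their children, and spawns a thunder-ball hit emitter at its location.
; For a locally controlled avatar it also calls the HUD's interface fade-in.
; The graph never ends the ability or restores the avatar.
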(event Ability|EventActivateAbility
  (bind _returnvalue (Ability|GetAvatarActorfromActorInfo))
  (Variables|/Script/Engine.Actor|SetCustomTimeDilation _returnvalue 0.0)
  (Utilities|FlowControl|Sequence
    (:then_0
      (for _array_element (Actor|GetComponentsByClass _returnvalue "/Script/Engine.SkeletalMeshComponent")
        (Rendering|SetVisibility _array_element false true)))
    (:then_1
      (Effects|SpawnEmitteratLocation "/Game/ExternalResource/FXVarietyPack/Particles/P_ky_ThunderBallHit.P_ky_ThunderBallHit" (Transformation|GetActorLocation (Ability|GetAvatarActorfromActorInfo))))
    (:then_2
      (Pawn|IsLocallyControlled
        (:True
          (Class|IBPSTHUDInterface|FadeinOutInterface(Message) (HUD|GetHUD (Game|GetPlayerController 0)) true 2.0 false))))))