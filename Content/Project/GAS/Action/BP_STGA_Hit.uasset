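; Gameplay ability on the defender that resolves incoming hits into Hit, Guard, Parry, Perfect Parry or Execution.
; On GA.Action.Hit, the server reads hit data tables, applies damage and effects, and chooses montage and knockback point.
; Hit and Guard play a cue and motion-warped montage, while parries and executions hand off to other abilities on both fighters.
; The result syncs to the client, which replays only Hit.
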(event Custom|ProcessHit
  (params (Montage :type Anim%20Montage%20Object%20Reference) (KnockbackLoc :type Vector) (HitInfo :type Hit%20Param%20Structure%20%28by%20ref%29) (Attacker :type Actor%20Object%20Reference))
  (bind (_hittype _hitcue) (Utilities|Struct|BreakHitParam HitInfo))
  (Utilities|FlowControl|Sequence
    (:then_0
      (Class|GameplayAbility|ExecuteGameplayCuewithParams _hitcue (Ability|GameplayCue|MakeGameplayCueParameters :AggregatedSourceTags (GameplayTags|MakeGameplayTagContainerfromArray (Utilities|Array|MakeArray _hittype)) :Instigator Attacker :EffectCauser (Ability|GetAvatarActorfromActorInfo))))
    (:then_1
      (Class|MotionWarpingComponent|AddorUpdateWarpTargetfromLocationandRotation (Actor|GetComponentbyClass (Ability|GetAvatarActorfromActorInfo) "/Script/ProjectST.STMotionWarpingComponent") "Knockback" KnockbackLoc (Math|Rotator|MakeRotator 0.0 0.0 (.Yaw (Math|Rotator|BreakRotator (Math|Rotator|FindLookatRotation KnockbackLoc (Transformation|GetActorLocation (Ability|GetAvatarActorfromActorInfo)))))))
      (|PlayMontageandWaitProxy "Hit" Montage 1.0 "None" true 1.0 0.0 false
        (:OnCompleted
          _)
        (:OnInterrupted
          _)
        (:OnCancelled
          _))
      (Ability|EndAbility))))

(event Custom|ProcessHit_Client
  (params (Montage :type Anim%20Montage%20Object%20Reference) (KnockbackLoc :type Vector%20Net%20Quantize%20Structure) (HitParamIndex :type Integer) (Attacker :type Actor%20Object%20Reference))
  (bind _returnvalue (Utilities|GetDataTableRow "/Game/Project/TableData/HitParamTable.HitParamTable" (Utilities|String|StringToName (Utilities|String|ToString(Integer) HitParamIndex)))
    (:then
      (CallFunction|ProcessHit Montage KnockbackLoc _returnvalue Attacker))))

(event Ability|EventActivateAbility
  (bind _returnvalue (Ability|GetAvatarActorfromActorInfo))
  (Ability|HasAuthority
    (:True
      (bind _payload (Ability|Async|WaitGameplayEventToActor (Ability|GetAvatarActorfromActorInfo) "(TagName=\"GA.Action.Hit\")" true)
        (:EventReceived
          (Variables|Default|SetPayload _payload)
          (bind (_result _defenderanim _localchosenhitparam _hitparamindex) (CallFunction|ProcessDamage (.Instigator (Utilities|Struct|BreakGameplayEventData _payload)) (.Target (Utilities|Struct|BreakGameplayEventData _payload)) (.OptionalObject (Utilities|Struct|BreakGameplayEventData _payload))))
          (Variables|Default|SetHitParam _localchosenhitparam)
          (Variables|Default|SetDefenderHitAnim _defenderanim)
          (Variables|Default|SetHit%20Param%20Index _hitparamindex)
          (bind _output_get (Variables|Default|SetResult _result))
          (switch Utilities|FlowControl|Switch|SwitchonEDamagingResultType _output_get
            (:NewEnumerator0
              (bind _loc (CallFunction|CalculateKnockback (Variables|Default|GetHitParam) (.Instigator (Utilities|Struct|BreakGameplayEventData (Variables|Default|GetPayload))) (.Target (Utilities|Struct|BreakGameplayEventData (Variables|Default|GetPayload))) :!label _label))
              (Variables|Default|SetKnockbackLoc _loc)
              (|SyncNetDataGenericData "ServerGiveData" (Utilities|Struct|MakeSTGenericGameplayAbilityTargetDataParams (Utilities|Array|MakeArray (Utilities|Struct|BreakGameplayEventData (Variables|Default|GetPayload)) (Variables|Default|GetDefenderHitAnim)) (Utilities|Array|MakeArray (Variables|Default|GetKnockbackLoc)) (Utilities|Array|MakeArray (Variables|Default|GetResult)) (Utilities|Array|MakeArray (Variables|Default|GetHit%20Param%20Index)))
                (:OnSync
                  (CallFunction|ProcessHit (Variables|Default|GetDefenderHitAnim) (Variables|Default|GetKnockbackLoc) (Variables|Default|GetHitParam) (Utilities|Struct|BreakGameplayEventData (Variables|Default|GetPayload))))))
            (:NewEnumerator2
              (goto _label))
            (:NewEnumerator3
              (bind _returnvalue_2 (Game|ConstructObjectfromClass (Ability|GetAvatarActorfromActorInfo) "/Game/Project/GAS/Action/BP_HitInfoObject.BP_HitInfoObject_C" (Utilities|Struct|BreakHitParam (Variables|Default|GetHitParam))))
              (Variables|Default|SetHitInfoObject _returnvalue_2)
              (Abilities|TryActivateAbilitybyClass (Ability|GetAbilitySystemComponent _returnvalue) "/Game/Project/GAS/Combat/BP_STGA_Katana_Parry.BP_STGA_Katana_Parry_C" true :!label _label_2)
              (Ability|SendGameplayEventtoActor _returnvalue "(TagName=\"GA.Action.Parry\")" (Utilities|Struct|MakeGameplayEventData (.Instigator (Utilities|Struct|BreakGameplayEventData (Variables|Default|GetPayload))) (.Target (Utilities|Struct|BreakGameplayEventData (Variables|Default|GetPayload))) (Variables|Default|GetHitInfoObject)))
              (Abilities|TryActivateAbilitybyClass (Ability|GetAbilitySystemComponent (Utilities|Struct|BreakGameplayEventData (Variables|Default|GetPayload))) "/Game/Project/GAS/Action/BP_STGA_Parried.BP_STGA_Parried_C" true)
              (Ability|SendGameplayEventtoActor (Utilities|Struct|BreakGameplayEventData (Variables|Default|GetPayload)) "(TagName=\"GA.Action.Parried\")" (Utilities|Struct|MakeGameplayEventData (.Instigator (Utilities|Struct|BreakGameplayEventData (Variables|Default|GetPayload))) (.Target (Utilities|Struct|BreakGameplayEventData (Variables|Default|GetPayload))) (Variables|Default|GetHitInfoObject)))
              (|SyncNetDataGenericData "ServerGiveData" (Utilities|Struct|MakeSTGenericGameplayAbilityTargetDataParams (Utilities|Array|MakeArray (Variables|Default|GetResult))) :!label _label_3
                (:OnSync
                  (Ability|EndAbility))))
            (:NewEnumerator4
              (bind _returnvalue_3 (Game|ConstructObjectfromClass (Ability|GetAvatarActorfromActorInfo) "/Game/Project/GAS/Action/BP_HitInfoObject.BP_HitInfoObject_C" (Utilities|Struct|BreakHitParam (Variables|Default|GetHitParam)) true))
              (Variables|Default|SetHitInfoObject _returnvalue_3)
              (goto _label_2))
            (:NewEnumerator6
              (Abilities|TryActivateAbilitybyClass (Ability|GetAbilitySystemComponent (Utilities|Struct|BreakGameplayEventData (Variables|Default|GetPayload))) "/Game/Project/GAS/Combat/BP_STGA_Katana_Execution.BP_STGA_Katana_Execution_C" true)
              (Ability|SendGameplayEventtoActor (Utilities|Struct|BreakGameplayEventData (Variables|Default|GetPayload)) "(TagName=\"GA.Execution\")" (Utilities|Struct|MakeGameplayEventData (.Instigator (Utilities|Struct|BreakGameplayEventData (Variables|Default|GetPayload))) (.Target (Utilities|Struct|BreakGameplayEventData (Variables|Default|GetPayload))) (Math|Conversions|ToFloat(Integer) (Utilities|Struct|BreakHitParam (Variables|Default|GetHitParam)))))
              (Abilities|TryActivateAbilitybyClass (Ability|GetAbilitySystemComponentfromActorInfo) "/Game/Project/GAS/Action/BP_STGA_Dead.BP_STGA_Dead_C" true)
              (Ability|SendGameplayEventtoActor (Ability|GetAvatarActorfromActorInfo) "(TagName=\"GA.Action.Dead\")" (Utilities|Struct|MakeGameplayEventData "/Game/Project/Character/Animation/ProcessedAnimation/Execution/ARPG_Samurai_Anim_UE_Executed_Death_Montage.ARPG_Samurai_Anim_UE_Executed_Death_Montage"))
              (goto _label_3))))))
    (:False
      (bind _data (|SyncNetDataGenericData "ServerGiveData" (Utilities|Struct|MakeSTGenericGameplayAbilityTargetDataParams))
        (:OnSync
          (Variables|Default|SetClientData _data)
          (switch Utilities|FlowControl|Switch|SwitchonEDamagingResultType (Utilities|Enum|ByteToEnumEDamagingResultType (Utilities|Array|Get(acopy) (.Enums (Utilities|Struct|BreakSTGenericGameplayAbilityTargetDataParams (Variables|Default|GetClientData)))))
            (:NewEnumerator0
              (bind _as액터 (Utilities|Casting|CastToActor (Utilities|Array|Get(acopy) (.Objects (Utilities|Struct|BreakSTGenericGameplayAbilityTargetDataParams (Variables|Default|GetClientData))))))
              (bind _as애님_몽타주 (Utilities|Casting|CastToAnimMontage (Utilities|Array|Get(acopy) (.Objects (Utilities|Struct|BreakSTGenericGameplayAbilityTargetDataParams (Variables|Default|GetClientData))) 1)))
              (CallFunction|ProcessHitClient _as애님_몽타주 (Math|Vector|MakeVectorNetQuantize (.x (Utilities|Array|Get(acopy) (.Vectors (Utilities|Struct|BreakSTGenericGameplayAbilityTargetDataParams (Variables|Default|GetClientData))))) (.y (Utilities|Array|Get(acopy) (.Vectors (Utilities|Struct|BreakSTGenericGameplayAbilityTargetDataParams (Variables|Default|GetClientData))))) (.z (Utilities|Array|Get(acopy) (.Vectors (Utilities|Struct|BreakSTGenericGameplayAbilityTargetDataParams (Variables|Default|GetClientData)))))) (Utilities|Array|Get(acopy) (.Ints (Utilities|Struct|BreakSTGenericGameplayAbilityTargetDataParams (Variables|Default|GetClientData)))) _as액터))
            (:NewEnumerator2
              (Ability|EndAbility :!label _label_4))
            (:NewEnumerator3
              (goto _label_4))
            (:NewEnumerator4
              (goto _label_4))
            (:NewEnumerator6
              (goto _label_4))))))))

(event Ability|EventOnEndAbility
  (params (bWasCancelled :type Boolean)))

(fn ProcessDamaging
  (params (HitParam :type Hit%20Param%20Structure%20%28by%20ref%29) (Attacker :type Actor%20Object%20Reference) (Defender :type Actor%20Object%20Reference))
  (bind (_bsuccessfullyfoundattribute _returnvalue) (Ability|Attribute|GetFloatAttribute Defender "(AttributeName=\"CurrentHealth\",Attribute=/Script/ProjectST.STAttributeSet:CurrentHealth,AttributeOwner=\"/Script/CoreUObject.Class'/Script/ProjectST.STAttributeSet'\")"))
  (bind _returnvalue_2 (Class|STStateInterface|GetStates(Message) Defender))
  (LocalVariables|SetLocalDefenderState _returnvalue_2)
  (bind _result (CallFunction|GetCurrentDamagingType Defender Attacker))
  (bind _output_get (LocalVariables|SetLocalDamagingResult _result))
  (switch Utilities|FlowControl|Switch|SwitchonEDamagingResultType _output_get
    (:NewEnumerator0
      (bind _returnvalue_3 (Spec|MakeSpecHandle(ByClass) "/Game/Project/GAS/Effect/BP_STGE_Hit.BP_STGE_Hit_C" Attacker Defender))
      (bind _returnvalue_4 (Ability|GameplayEffect|AssignTagSetbyCallerMagnitude _returnvalue_3 "(TagName=\"EC.Damage\")" (.BaseDamage (Utilities|Struct|BreakHitParam HitParam))))
      (Ability|ApplyGameplayEffectSpecToOwner _returnvalue_4)
      (if (and (<= _returnvalue 0.0) _bsuccessfullyfoundattribute)
        (bind _returnvalue_5 (Utilities|GetDataTableRow "/Game/Project/TableData/ExecutionInfoTable.ExecutionInfoTable" (Utilities|String|StringToName (Utilities|String|ToString(Integer) (.ExecutionTableRow (Utilities|Struct|BreakHitParam HitParam)))))
          (:then
            (LocalVariables|SetLocalDamagingResult "NewEnumerator6")
            (bind _returnvalue_6 (Class|STStateInterface|HasState(Message) Attacker (GameplayTags|MakeLiteralGameplayTag "(TagName=\"State.Falling\")")))
            (bind _returnvalue_7 (Class|STStateInterface|HasState(Message) Defender (GameplayTags|MakeLiteralGameplayTag "(TagName=\"State.Falling\")")))
            (if (or _returnvalue_6 _returnvalue_7)
              _
              (else
                (return (Utilities|Struct|BreakExecutionInfo _returnvalue_5) true (LocalVariables|GetLocalDamagingResult)))))
          (:RowNotFound
            _))
        (return 0 true (LocalVariables|GetLocalDamagingResult))
        (else
          (CallFunction|OnHitSuccees HitParam)
          (bind _montage (CallFunction|SelectHitMontage Defender HitParam))
          (return _montage false (LocalVariables|GetLocalDamagingResult)))))
    (:NewEnumerator2
      (return "/Game/Project/Character/Animation/ProcessedAnimation/Hit/ARPG_Samurai_Anim_UE_Guard_Hit3_Montage.ARPG_Samurai_Anim_UE_Guard_Hit3_Montage" false (LocalVariables|GetLocalDamagingResult)))
    (:NewEnumerator3
      (return 0 false (LocalVariables|GetLocalDamagingResult)))
    (:NewEnumerator4
      (return 0 false (LocalVariables|GetLocalDamagingResult)))))

(fn SelectHitMontage
  (params (Defender :type Actor%20Object%20Reference) (HitParam :type Hit%20Param%20Structure%20%28by%20ref%29))
  (Utilities|FlowControl|Sequence
    (:then_0
      (bind _returnvalue (Class|STStateInterface|HasState(Message) Defender (GameplayTags|MakeLiteralGameplayTag "(TagName=\"State.Falling\")")))
      (if _returnvalue
        (if (!= (Utilities|Struct|BreakHitParam HitParam) "(TagName=\"Hit.KnockDown\")")
          (return "/Game/Project/Character/Animation/ProcessedAnimation/Hit/Fly/ARPG_Samurai_Anim_UE_Death_Airborne_Start_Montage.ARPG_Samurai_Anim_UE_Death_Airborne_Start_Montage"))))
    (:then_1
      (bind _returnvalue_2 (Class|STStateInterface|HasState(Message) Defender (GameplayTags|MakeLiteralGameplayTag "(TagName=\"State.Lying\")")))
      (if _returnvalue_2
        (return "/Game/Project/Character/Animation/ProcessedAnimation/Hit/Fly/ARPG_Samurai_Anim_UE_Death_Airborne_Start_Montage.ARPG_Samurai_Anim_UE_Death_Airborne_Start_Montage")))
    (:then_2
      (|SwitchGameplayTag (.HitType (Utilities|Struct|BreakHitParam HitParam))
        (:Default
          (return "/Game/Project/Character/Animation/ProcessedAnimation/Hit/ARPG_Samurai_Anim_UE_WeakKnockBack_Montage.ARPG_Samurai_Anim_UE_WeakKnockBack_Montage"))
        (:Hit.Head
          (return "/Game/Project/Character/Animation/ProcessedAnimation/Hit/ARPG_Samurai_Anim_UE_WeakKnockBack_Montage.ARPG_Samurai_Anim_UE_WeakKnockBack_Montage"))
        (:Hit.Left
          (return "/Game/Project/Character/Animation/ProcessedAnimation/Hit/ARPG_Samurai_Anim_UE_WeakKnockBack_Montage.ARPG_Samurai_Anim_UE_WeakKnockBack_Montage"))
        (:Hit.Right
          (return "/Game/Project/Character/Animation/ProcessedAnimation/Hit/ARPG_Samurai_Anim_UE_WeakKnockBack_Montage.ARPG_Samurai_Anim_UE_WeakKnockBack_Montage"))
        (:Hit.KnockDown
          (return (.OutItem (Utilities|Array|Random (Utilities|Array|MakeArray "/Game/Project/Character/Animation/ProcessedAnimation/Hit/ARPG_Samurai_Anim_UE_Hit_knockdown4_Montage.ARPG_Samurai_Anim_UE_Hit_knockdown4_Montage" "/Game/Project/Character/Animation/ProcessedAnimation/Hit/ARPG_Samurai_Anim_UE_Hit_knockdown_Montage.ARPG_Samurai_Anim_UE_Hit_knockdown_Montage")))))
        (:Hit.Flying
          (return "/Game/Project/Character/Animation/ProcessedAnimation/Hit/Fly/ARPG_Samurai_Anim_UE_Death_Airborne_Start_Montage.ARPG_Samurai_Anim_UE_Death_Airborne_Start_Montage"))
        (:Hit.Dicing
          (return "/Game/Project/Character/Animation/ProcessedAnimation/Hit/ARPG_Samurai_Anim_UE_Diced_Montage1.ARPG_Samurai_Anim_UE_Diced_Montage1"))))))

(fn CalculateKnockback
  (params (HitParam :type Hit%20Param%20Structure%20%28by%20ref%29) (Attacker :type Actor%20Object%20Reference) (Defender :type Actor%20Object%20Reference))
  (bind _knockbackdistance (Utilities|Struct|BreakHitParam HitParam))
  (Utilities|FlowControl|Sequence
    (:then_0
      (LocalVariables|SetLocalAttackerToDefenderVec (Class|KismetMathLibrary|VectorNormal2D (- (Transformation|GetActorLocation Defender) (Transformation|GetActorLocation Attacker)) 0.0001))
      (LocalVariables|SetLocalDefenderToAttackerVec (Class|KismetMathLibrary|VectorNormal2D (- (Transformation|GetActorLocation Attacker) (Transformation|GetActorLocation Defender)) 0.0001)))
    (:then_1
      (bind _returnvalue (Class|STStateInterface|GetStates(Message) Defender))
      (LocalVariables|SetLocalShouldDecreaseKnockBackDistance (GameplayTags|HasAnyTags _returnvalue (GameplayTags|MakeLiteralGameplayTagContainer "(GameplayTags=((TagName=\"CombatState.Guard\"),(TagName=\"State.Lying\")))") true)))
    (:then_2
      (LocalVariables|SetLocalKnockbackDistance (select (LocalVariables|GetLocalShouldDecreaseKnockBackDistance) (* _knockbackdistance 0.35) _knockbackdistance)))
    (:then_3
      (bind _returnvalue_2 (Class|STStateInterface|HasState(Message) Defender (GameplayTags|MakeLiteralGameplayTag "(TagName=\"State.Falling\")")))
      (if _returnvalue_2
        (LocalVariables|SetLocalOrigin (Transformation|GetActorLocation Defender))
        (LocalVariables|SetLocalVerticalVector "0.000000,0.000000,-75.000000")
        (LocalVariables|SetLocalKnockbackDistance (* (LocalVariables|GetLocalKnockbackDistance) 1.5))))
    (:then_5
      (|SwitchGameplayTag (Utilities|Struct|BreakHitParam HitParam)
        (:Default
          (LocalVariables|SetLocalOrigin (Transformation|GetActorLocation Defender)))
        (:Knockback.Pull
          (LocalVariables|SetLocalOrigin (Transformation|GetActorLocation Defender))
          (LocalVariables|SetLocalHorizontalVector (* (LocalVariables|GetLocalDefenderToAttackerVec) (LocalVariables|GetLocalKnockbackDistance))))
        (:Knockback.PullToHitter
          (if (LocalVariables|GetLocalShouldDecreaseKnockBackDistance)
            (LocalVariables|SetLocalOrigin (Transformation|GetActorLocation Defender))
            (else
              (LocalVariables|SetLocalOrigin (Transformation|GetActorLocation Attacker))
              (LocalVariables|SetLocalHorizontalVector (* (Transformation|GetActorForwardVector Attacker) 1.5e+02)))))
        (:Knockback.Push
          (LocalVariables|SetLocalOrigin (Transformation|GetActorLocation Defender))
          (LocalVariables|SetLocalHorizontalVector (* (LocalVariables|GetLocalAttackerToDefenderVec) (LocalVariables|GetLocalKnockbackDistance))))
        (:Knockback.Fly
          (LocalVariables|SetLocalOrigin (Transformation|GetActorLocation Defender))
          (LocalVariables|SetLocalHorizontalVector (* (LocalVariables|GetLocalAttackerToDefenderVec) 5e+01))
          (if (Math|Vector|VectorIsNearlyZero (LocalVariables|GetLocalVerticalVector))
            (if (not (LocalVariables|GetLocalShouldDecreaseKnockBackDistance))
              (LocalVariables|SetLocalVerticalVector (Math|Vector|MakeVector 0.0 0.0 (LocalVariables|GetLocalKnockbackDistance))))
            (else
              (LocalVariables|SetLocalVerticalVector (+ (LocalVariables|GetLocalVerticalVector) (Math|Vector|MakeVector 0.0 0.0 (Utilities|Struct|BreakHitParam HitParam)))))))))
    (:then_6
      (return (+ (LocalVariables|GetLocalOrigin) (LocalVariables|GetLocalVerticalVector) (LocalVariables|GetLocalHorizontalVector))))))

(fn ProcessDamage
  (params (Attacker :type Actor%20Object%20Reference) (Defender :type Actor%20Object%20Reference) (object :type Object%20Object%20Reference))
  (bind _asbp_hit_info_object (Utilities|Casting|CastToBP_HitInfoObject object)
    (:then
      (LocalVariables|SetLocalHitParamIndex (Variables|/Game/Project/GAS/Action/BP_HitInfoObject.BP_HitInfoObject_C|GetHitParam _asbp_hit_info_object))
      (bind _returnvalue (Utilities|GetDataTableRow "/Game/Project/TableData/HitParamTable.HitParamTable" (Utilities|String|StringToName (Utilities|String|ToString(Integer) (LocalVariables|GetLocalHitParamIndex))))
        (:then
          (bind _output_get (LocalVariables|SetLocalHitParam _returnvalue))
          (bind (_hitmontage _istargetdead _damagingresult) (CallFunction|ProcessDamaging _output_get Attacker Defender))
          (LocalVariables|SetLocalTargetDead _istargetdead)
          (LocalVariables|SetLocalDefenderChosenAnim _hitmontage)
          (LocalVariables|SetLocalResult _damagingresult)
          (return (LocalVariables|GetLocalResult) (LocalVariables|GetLocalDefenderChosenAnim) (LocalVariables|GetLocalHitParam) (LocalVariables|GetLocalHitParamIndex)))
        (:RowNotFound
          (return "NewEnumerator0" 0 "" 0))))
    (:CastFailed
      (return "NewEnumerator0" 0 "" 0))))

(fn GetCurrentDamagingType
  (params (Defender :type Actor%20Object%20Reference) (Attacker :type Actor%20Object%20Reference))
  (bind _returnvalue (Transformation|GetActorForwardVector Defender))
  (bind _returnvalue_2 (Transformation|GetActorForwardVector Attacker))
  (bind _returnvalue_3 (Math|Vector|NegateVector _returnvalue))
  (bind _returnvalue_4 (Class|KismetMathLibrary|VectorCosineAngle2D _returnvalue_2 _returnvalue_3))
  (bind _returnvalue_5 (Math|Trig|RadiansToDegrees _returnvalue_4))
  (bind _returnvalue_6 (Class|STStateInterface|GetStates(Message) Defender))
  (LocalVariables|SetLocalDefenderState _returnvalue_6)
  (LocalVariables|SetLocalDamagingResult "NewEnumerator0")
  (Utilities|FlowControl|Sequence
    (:then_0
      (if (GameplayTags|HasTag (LocalVariables|GetLocalDefenderState) "(TagName=\"CombatState.Guard\")")
        (if (and (<= _returnvalue_5 8e+01) (> _returnvalue_5 0.0))
          (LocalVariables|SetLocalDamagingResult "NewEnumerator2"))))
    (:then_1
      (if (GameplayTags|HasTag (LocalVariables|GetLocalDefenderState) "(TagName=\"CombatState.Parry\")")
        (LocalVariables|SetLocalDamagingResult "NewEnumerator3")))
    (:then_2
      (if (GameplayTags|HasTag (LocalVariables|GetLocalDefenderState) "(TagName=\"CombatState.PerfectParry\")")
        (LocalVariables|SetLocalDamagingResult "NewEnumerator4")))
    (:then_3
      (return (LocalVariables|GetLocalDamagingResult)))))

(fn OnHitSuccees
  (params (HitParam :type Hit%20Param%20Structure))
  (bind _payload (Variables|Default|GetPayload))
  (bind _payload_2 (Variables|Default|GetPayload))
  (bind (_instigator _target) (Utilities|Struct|BreakGameplayEventData _payload))
  (bind (_instigator_2 _target_2) (Utilities|Struct|BreakGameplayEventData _payload_2))
  (bind _returnvalue (Utilities|GetDataTableRow "/Game/Project/TableData/OnHitEffectTable.OnHitEffectTable" (Utilities|String|StringToName (Utilities|String|ToString(Integer) (Utilities|Struct|BreakHitParam HitParam))))
    (:then
      (LocalVariables|SetLocalOnHitEffect _returnvalue)
      (Utilities|FlowControl|Sequence
        (:then_0
          (if (Utilities|IsValidClass (Utilities|Struct|BreakOnHitEffectInfo (LocalVariables|GetLocalOnHitEffect)))
            (bind _returnvalue_2 (Spec|MakeSpecHandle(ByClass) (Utilities|Struct|BreakOnHitEffectInfo (LocalVariables|GetLocalOnHitEffect)) _instigator_2 _target_2))
            (Ability|ApplyGameplayEffectSpecToOwner _returnvalue_2)))
        (:then_1
          (if (Utilities|IsValidClass (Utilities|Struct|BreakOnHitEffectInfo (LocalVariables|GetLocalOnHitEffect)))
            (bind _returnvalue_3 (Spec|MakeSpecHandle(ByClass) (Utilities|Struct|BreakOnHitEffectInfo (LocalVariables|GetLocalOnHitEffect)) _instigator _target))
            (GameplayEffects|ApplyGameplayEffectSpecToSelf (Ability|GetAbilitySystemComponent (Utilities|Struct|BreakGameplayEventData (Variables|Default|GetPayload))) _returnvalue_3)))))))