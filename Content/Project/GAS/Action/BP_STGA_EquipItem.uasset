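; Gameplay ability that equips an item by spawning its actor on the avatar.
; On activation it waits for the GA.Action.Equip event and reads the equip data object from the payload.
; It synchronously loads the item actor class, spawns it, and snaps it to a socket on the avatar's second skeletal mesh.
; It then initializes the actor with item and equip data and ends, though failed casts leave the ability running.
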(event Ability|EventActivateAbility
  (bind _payload (Ability|Tasks|WaitGameplayEvent "(TagName=\"GA.Action.Equip\")" 0)
    (:EventReceived
      (bind _asbp_equip_data_object (Utilities|Casting|CastToBP_EquipDataObject (Utilities|Struct|BreakGameplayEventData _payload)))
      (bind _returnvalue (Utilities|LoadClassAssetBlocking (.EquipActorClass (Utilities|Struct|BreakItemEquipInfoData (Variables|/Game/Project/GAS/Action/BP_EquipDataObject.BP_EquipDataObject_C|GetEquipData _asbp_equip_data_object)))))
      (bind _asstequip_item_actor (Utilities|Casting|CastToSTEquipItemActorClass _returnvalue))
      (bind _returnvalue_2 (Game|SpawnActorfromClass _asstequip_item_actor (Math|Transform|MakeTransform "0, 0, 0" "0, 0, 0" "1.000000,1.000000,1.000000") "AlwaysSpawn" "MultiplyWithRoot" (Ability|GetAvatarActorfromActorInfo) 0))
      (Utilities|IsValid _returnvalue_2
        (:Is%20Valid
          (Transformation|AttachComponentToComponent _returnvalue_2 (Utilities|Array|Get(acopy) (Actor|GetComponentsByClass (Ability|GetAvatarActorfromActorInfo) "/Script/Engine.SkeletalMeshComponent") 1) (.SocketName (Utilities|Struct|BreakItemEquipInfoData (Variables|/Game/Project/GAS/Action/BP_EquipDataObject.BP_EquipDataObject_C|GetEquipData _asbp_equip_data_object))) "SnapToTarget" "SnapToTarget" "SnapToTarget" true)
          (Class|STEquipItemActor|Initialize _returnvalue_2 (Ability|GetAvatarActorfromActorInfo) (Variables|/Game/Project/GAS/Action/BP_EquipDataObject.BP_EquipDataObject_C|GetItemData _asbp_equip_data_object) (Variables|/Game/Project/GAS/Action/BP_EquipDataObject.BP_EquipDataObject_C|GetEquipData _asbp_equip_data_object))
          (Ability|EndAbility))
        (:Is%20Not%20Valid
          (Ability|EndAbility))))))

(event Ability|EventOnEndAbility
  (params (bWasCancelled :type Boolean)))