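; Gameplay ability for the reaction of a character whose action gets parried, snapping it to face the parrier and playing a guard-break montage.
; On activation the server waits once for the GA.Action.Parried event, then passes the payload's target to the non-authority side through a server-to-client data sync.
; Both sides run ProcessParried with that actor, and the ability ends when the montage completes, blends out or is interrupted.
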(event Custom|ProcessParried
  (params (Parrier :type Actor%20Object%20Reference))
  (Transformation|SetActorRotation (Ability|GetAvatarActorfromActorInfo) (Math|Rotator|FindLookatRotation (Transformation|GetActorLocation (Ability|GetAvatarActorfromActorInfo)) (Transformation|GetActorLocation Parrier)) true)
  (Utilities|FlowControl|Sequence
    (:then_1
      (|PlayMontageandWaitProxy "Parry" "/Game/Project/Character/Animation/ProcessedAnimation/Parry/ARPG_Samurai_Anim_UE_Guard_Break_Montage.ARPG_Samurai_Anim_UE_Guard_Break_Montage" 1.0 "None" true 1.0 0.0 false
        (:OnCompleted
          _)
        (:OnBlendOut
          _)
        (:OnInterrupted
          _)
        (:OnCancelled
          _))
      (Ability|EndAbility))))

(event Ability|EventActivateAbility
  (Ability|HasAuthority
    (:True
      (bind _payload (Ability|Async|WaitGameplayEventToActor (Ability|GetAvatarActorfromActorInfo) "(TagName=\"GA.Action.Parried\")" true)
        (:EventReceived
          (bind _data (|SyncNetDataGenericData "ServerGiveData" (Utilities|Struct|MakeSTGenericGameplayAbilityTargetDataParams "(GameplayTags=)" (Utilities|Array|MakeArray (.Target (Utilities|Struct|BreakGameplayEventData _payload)))))
            (:OnSync
              (bind _as액터 (Utilities|Casting|CastToActor (Utilities|Array|Get(acopy) (.Objects (Utilities|Struct|BreakSTGenericGameplayAbilityTargetDataParams _data)))))
              (CallFunction|ProcessParried _as액터))))))
    (:False
      (bind _data_2 (|SyncNetDataGenericData "ServerGiveData")
        (:OnSync
          (bind _as액터_2 (Utilities|Casting|CastToActor (Utilities|Array|Get(acopy) (.Objects (Utilities|Struct|BreakSTGenericGameplayAbilityTargetDataParams _data_2)))))
          (CallFunction|ProcessParried _as액터_2))))))

(event Ability|EventOnEndAbility
  (params (bWasCancelled :type Boolean)))