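; Gameplay ability for a samurai sway: an eight-way evade from movement input, or a short backward dodge without input.
; The locally controlled side snaps camera-relative input to eight directions, picking a montage and warp distance.
; It plays the sway immediately and sends target, montage and yaw to a server event, which commits before playing.
; Sway faces control yaw, sets a motion warp target, and ends with the montage.
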(event Custom|Sway
  (params (TargetLoc :type Vector) (PickedSway :type Anim%20Montage%20Object%20Reference) (InitialRot :type Float%20%28double-precision%29))
  (Transformation|SetActorRotation (Ability|GetAvatarActorfromActorInfo) (Math|Rotator|MakeRotator 0.0 0.0 InitialRot) true)
  (Class|MotionWarpingComponent|AddorUpdateWarpTargetfromLocationandRotation (Actor|GetComponentbyClass (Ability|GetAvatarActorfromActorInfo) "/Script/MotionWarping.MotionWarpingComponent") "Sway" TargetLoc (Math|Rotator|MakeRotator 0.0 0.0 InitialRot))
  (|PlayMontageandWaitProxy "Sway" PickedSway 1.0 "None" true 1.0 0.0 false
    (:OnBlendOut
      _)
    (:OnInterrupted
      _)
    (:OnCancelled
      _))
  (Ability|EndAbility))

(event Custom|Sway_Server
  (params (TargetLocation :type Vector) (MontageToPlay :type Anim%20Montage%20Object%20Reference) (InitialRot :type Float%20%28double-precision%29))
  (bind _returnvalue (Ability|CommitAbility))
  (if _returnvalue
    (CallFunction|Sway TargetLocation MontageToPlay InitialRot)))

(event Ability|EventActivateAbility
  (Pawn|IsLocallyControlled
    (:True
      (bind _as캐릭터 (Utilities|Casting|CastToCharacter (Ability|GetAvatarActorfromActorInfo)))
      (if (Math|Vector|VectorIsNearlyZero (Pawn|Components|PawnMovement|GetLastInputVector (Variables|/Script/Engine.Character|GetCharacterMovement _as캐릭터)))
        (bind _output_get (Variables|Default|SetClosest%20Vector "(X=-1.000000,Y=0.000000)"))
        (bind (_targetloc _pickedsway _initialrot) (CallFunction|PrepareSway _output_get true))
        (CallFunction|SwayServer _targetloc _pickedsway _initialrot)
        (CallFunction|Sway _targetloc _pickedsway _initialrot)
        (else
          (bind _output_get_2 (Variables|Default|SetClosest%20Vector (CallFunction|GetClosest8Direction (Math|Conversions|ToVector2D(Vector) (Class|KismetMathLibrary|VectorNormal2D (Math|Vector|UnrotateVector (Pawn|Components|PawnMovement|GetLastInputVector (Variables|/Script/Engine.Character|GetCharacterMovement _as캐릭터)) (Camera|GetCameraRotation (Variables|/Script/Engine.PlayerController|GetPlayerCameraManager (Game|GetPlayerController 0)))) 0.0001)))))
          (bind (_targetloc_2 _pickedsway_2 _initialrot_2) (CallFunction|PrepareSway _output_get_2 false))
          (CallFunction|SwayServer _targetloc_2 _pickedsway_2 _initialrot_2)
          (CallFunction|Sway _targetloc_2 _pickedsway_2 _initialrot_2))))))

(event Ability|EventOnEndAbility
  (params (bWasCancelled :type Boolean)))

(fn PickSway
  (params (Input :type Vector%202D%20Structure) (IsDodge :type Boolean))
  (bind (_x _y) (Math|Vector2D|BreakVector2D Input))
  (Utilities|FlowControl|Sequence
    (:then_0
      (if IsDodge
        ;[0.15 0.15 0.15 0.5] Nothing -> Dodge
        (return "/Game/Project/Character/Animation/ProcessedAnimation/Evade/ARPG_Samurai_Anim_UE_Dodge_Montage.ARPG_Samurai_Anim_UE_Dodge_Montage" 2e+02)))
    (:then_1
      (if (> _x 0.5)
        (LocalVariables|SetIsForward true)
        (elif (< _x -0.5)
          (LocalVariables|SetIsBackward true))))
    (:then_2
      (if (> _y 0.5)
        (LocalVariables|SetIsRight true)
        (elif (< _y -0.5)
          (LocalVariables|SetIsLeft true))))
    (:then_3
      (if (LocalVariables|GetIsForward)
        (if (LocalVariables|GetIsRight)
          ;[0.15 0.15 0.15 0.5] FR
          (return "/Game/Project/Character/Animation/ProcessedAnimation/Evade/ARPG_Samurai_Anim_UE_Evade_Forward_Right_Montage.ARPG_Samurai_Anim_UE_Evade_Forward_Right_Montage" 4e+02)
          (elif (LocalVariables|GetIsLeft)
            ;[0.15 0.15 0.15 0.5] FL
            (return "/Game/Project/Character/Animation/ProcessedAnimation/Evade/ARPG_Samurai_Anim_UE_Evade_Forward_Left_Montage.ARPG_Samurai_Anim_UE_Evade_Forward_Left_Montage" 4e+02)
            (else
              ;[0.15 0.15 0.15 0.5] F
              (return "/Game/Project/Character/Animation/ProcessedAnimation/Evade/ARPG_Samurai_Anim_UE_Evade_Forward_Montage.ARPG_Samurai_Anim_UE_Evade_Forward_Montage" 4.5e+02))))
        (elif (LocalVariables|GetIsBackward)
          (if (LocalVariables|GetIsRight)
            ;[0.15 0.15 0.15 0.5] BR
            (return "/Game/Project/Character/Animation/ProcessedAnimation/Evade/ARPG_Samurai_Anim_UE_Evade_Backward_Right_Montage.ARPG_Samurai_Anim_UE_Evade_Backward_Right_Montage" 4e+02)
            (elif (LocalVariables|GetIsLeft)
              ;[0.15 0.15 0.15 0.5] BL
              (return "/Game/Project/Character/Animation/ProcessedAnimation/Evade/ARPG_Samurai_Anim_UE_Evade_Backward_Left_Montage.ARPG_Samurai_Anim_UE_Evade_Backward_Left_Montage" 4e+02)
              (else
                ;[0.15 0.15 0.15 0.5] B
                (return "/Game/Project/Character/Animation/ProcessedAnimation/Evade/ARPG_Samurai_Anim_UE_Evade_Backward_Montage.ARPG_Samurai_Anim_UE_Evade_Backward_Montage" 4.5e+02))))
          (elif (LocalVariables|GetIsRight)
            ;[0.15 0.15 0.15 0.5] R
            (return "/Game/Project/Character/Animation/ProcessedAnimation/Evade/ARPG_Samurai_Anim_UE_Evade_Right_Montage.ARPG_Samurai_Anim_UE_Evade_Right_Montage" 4.5e+02)
            (elif (LocalVariables|GetIsLeft)
              ;[0.15 0.15 0.15 0.5] L
              (return "/Game/Project/Character/Animation/ProcessedAnimation/Evade/ARPG_Samurai_Anim_UE_Evade_Left_Montage.ARPG_Samurai_Anim_UE_Evade_Left_Montage" 4.5e+02))))))))

(fn AddVectortoLoc
  (params (Vector :type Vector) (Scalar :type Float%20%28double-precision%29))
  (return (+ (Transformation|GetActorLocation (Ability|GetAvatarActorfromActorInfo)) (* Vector Scalar))))

(fn GetClosest8Direction
  (params (Direction :type Vector%202D%20Structure))
  (for _array_element (Variables|Default|GetPredefinedDirections)
    (bind _output_get (LocalVariables|SetLocalDot (Math|Vector2D|DotProduct(2D) Direction _array_element)))
    (if (> _output_get 0.0)
      (if (> (LocalVariables|GetLocalDot) (LocalVariables|GetLocalClosestDot))
        (LocalVariables|SetLocalClosestDirection _array_element)
        (LocalVariables|SetLocalClosestDot (LocalVariables|GetLocalDot)))))
  (return (LocalVariables|GetLocalClosestDirection)))

(fn PrepareSway
  (params (ClosestVector :type Vector%202D%20Structure) (IsDodge :type Boolean))
  (bind _returnvalue (Game|GetPlayerController 0))
  (bind _returnvalue_2 (Pawn|GetControlRotation _returnvalue :!class /Script/Engine.Controller))
  (bind _yaw (Math|Rotator|BreakRotator _returnvalue_2))
  (bind (_pickedsway _warpingdistance) (CallFunction|PickSway ClosestVector IsDodge))
  (return (CallFunction|AddVectortoLoc (Math|Vector|RotateVector (Math|Conversions|ToVector(Vector2D) (Variables|Default|GetClosest%20Vector)) (Math|Rotator|MakeRotator 0.0 0.0 _yaw)) _warpingdistance) _pickedsway _yaw))