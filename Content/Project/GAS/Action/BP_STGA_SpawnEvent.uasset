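; Gameplay ability that plays a spawn event on its avatar: a gesture montage, plus a magic-circle particle effect on non-authority instances.
; On activation, the authority goes straight to the montage task, while other instances first spawn the emitter below the avatar, provided the avatar is valid.
; Montage completion, blend-out, interruption or cancellation ends the ability and deactivates any spawned emitter.
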(event Custom|ProcessSpawn
  (bind _returnvalue (Ability|GetAvatarActorfromActorInfo))
  (Ability|HasAuthority
    (:True
      _)
    (:False
      (Utilities|IsValid _returnvalue
        (:Is%20Valid
          (bind _returnvalue_2 (Effects|SpawnEmitteratLocation "/Game/ExternalResource/FXVarietyPack/Particles/P_ky_magicCircle1.P_ky_magicCircle1" (+ (Transformation|GetActorLocation _returnvalue) "0.000000,0.000000,-80.000000")))))))
  (|PlayMontageandWaitProxy "SpawnEvent" "/Game/Project/Character/Animation/ProcessedAnimation/CommonAction/SillyGesture04_Montage.SillyGesture04_Montage" 1.0 "None" true 1.0 0.0 false
    (:OnCompleted
      _)
    (:OnBlendOut
      _)
    (:OnInterrupted
      _)
    (:OnCancelled
      _))
  (Ability|EndAbility)
  (Utilities|IsValid _returnvalue_2
    (:Is%20Valid
      (Components|Activation|Deactivate _returnvalue_2))))

(event Ability|EventActivateAbility
  (CallFunction|ProcessSpawn))

(event Ability|EventOnEndAbility
  (params (bWasCancelled :type Boolean)))