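; Sprint gameplay ability that toggles the CombatState.Sprint state on the avatar according to the input trigger phase.
; When locally controlled, it commits, waits for one Input.InputInstance gameplay event and forwards the trigger phase from its ComboInputData payload to a server event.
; The server event commits again, then adds the state replication message on Started or Triggered and removes it on Completed.
; The ability ends after each processed input rather than staying active while sprinting.
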(event Custom|ProcessSprint
  (params (Selection :type ETriggerEvent%20Enum :default "None"))
  (switch Utilities|FlowControl|Switch|SwitchonETriggerEvent Selection
    (:Triggered
      (Class|STStateInterface|AddStateReplication(Message) (Ability|GetAvatarActorfromActorInfo) (GameplayTags|MakeLiteralGameplayTag "(TagName=\"CombatState.Sprint\")") :!label _label))
    (:Started
      (goto _label))
    (:Ongoing
      _)
    (:Canceled
      _)
    (:Completed
      (Class|STStateInterface|RemoveStateReplication(Message) (Ability|GetAvatarActorfromActorInfo) (GameplayTags|MakeLiteralGameplayTag "(TagName=\"CombatState.Sprint\")"))))
  (Ability|EndAbility))

(event Custom|ProcessSprint_Server
  (params (Selection :type ETriggerEvent%20Enum :default "None"))
  (bind _returnvalue (Ability|CommitAbility))
  (if _returnvalue
    (CallFunction|ProcessSprint Selection)
    (else
      (Ability|EndAbility))))

(event Ability|EventOnEndAbility
  (params (bWasCancelled :type Boolean)))

(event Ability|EventActivateAbility
  (Pawn|IsLocallyControlled
    (:True
      (bind _returnvalue (Ability|CommitAbility))
      (if _returnvalue
        (bind _payload (Ability|Tasks|WaitGameplayEvent "(TagName=\"Input.InputInstance\")" 0 true)
          (:EventReceived
            (bind _ascombo_input_data (Utilities|Casting|CastToComboInputData (Utilities|Struct|BreakGameplayEventData _payload))
              (:then
                (CallFunction|ProcessSprintServer (Utilities|Struct|BreakInputActionInstance (Variables|/Script/ProjectST.ComboInputData|GetInputInstance _ascombo_input_data))))
              (:CastFailed
                (Ability|EndAbility)))))
        (else
          (Ability|EndAbility))))))