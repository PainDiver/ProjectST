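; Enemy character Blueprint that lets a player open a status UI tied to the enemy's inventory through interaction.
; On BeginPlay it binds OnInteractionDone to the end-interaction delegate in the first entry of its interaction component.
; On a successful interaction by a locally controlled player character, it passes its inventory component in a BP_ShowWidget_Status object to the HUD, which is messaged by the UI.StatusBase tag.
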(event Custom|OnInteractionDone
  (params (Interactor :type Actor%20Object%20Reference) (bIsSuccess :type Boolean) (InteractionInfo :type Interaction%20Info%20Structure%20%28by%20ref%29))
  (bind _returnvalue (Game|GetPlayerController 0))
  (if bIsSuccess
    (bind _as캐릭터 (Utilities|Casting|CastToCharacter Interactor))
    (if (and (Pawn|IsLocallyControlled _as캐릭터) (Pawn|IsPlayerControlled _as캐릭터))
      (bind _returnvalue_2 (Game|ConstructObjectfromClass _returnvalue "/Game/Project/Character/Player/HUD/UIParam/BP_ShowWidget_Status.BP_ShowWidget_Status_C" "NewEnumerator3" (Class|STCharacterInterface|GetInventoryComponent)))
      (Class|IBPSTHUDInterface|ShowWidgetbyTagInterface(Message) (HUD|GetHUD _returnvalue) "(TagName=\"UI.StatusBase\")" _returnvalue_2))))

(event EventBeginPlay
  (|SetBy-RefVar (Utilities|Array|Get(acopy) (Variables|/Script/ProjectST.STInteractionObjectComponent|GetInteractionDelegates (Variables|Default|GetInteractionObjectComp))) (Utilities|Struct|MakeInteractionDelegateSets "(null).None" "(null).None" "(null).None" "(null).None" (EventDispatchers|CreateEvent :!event Custom|OnInteractionDone))))

(event Collision|EventActorBeginOverlap
  (params (OtherActor :type Actor%20Object%20Reference)))

(event EventTick
  (params (DeltaSeconds :type Float%20%28single-precision%29)))

(fn ConstructionScript)