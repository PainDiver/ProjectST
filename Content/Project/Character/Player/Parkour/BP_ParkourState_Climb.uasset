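; Parkour state that lets a character climb onto ledges, either from a walk or run or by catching them in the air.
; PrepareParkour sphere-traces forward for a wall, then downward for a top within climbable height, yielding body, hand and landing points.
; Only the first check after preparing starts gets full, speed-based reach; later ones use short air-catch reach.
; DoParkour activates the parkour ability and sends it points, ignored walls and montage via gameplay event.
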(event EventDoParkour
  (params (Owner :type Actor%20Object%20Reference) (ParkourPoints :type Array%20of%20Vectors) (WallsToIgnore :type Array%20of%20Primitive%20Component%20Object%20References))
  (Abilities|TryActivateAbilitybyClass (Ability|GetAbilitySystemComponent Owner) (Variables|Default|GetParkourGA) true)
  (bind _returnvalue (Game|ConstructObjectfromClass Owner "/Game/Project/Character/Player/Parkour/BP_ParkourData.BP_ParkourData_C" ParkourPoints WallsToIgnore (select (< (Math|Vector|VectorLengthXY (Transformation|GetVelocity Owner)) 4e+02) "/Game/Project/Character/Animation/ProcessedAnimation/Parkour/Climb/Parkour_Climb_Walk.Parkour_Climb_Walk" "/Game/Project/Character/Animation/ProcessedAnimation/Parkour/Climb/Parkour_Climb_Run.Parkour_Climb_Run") (Utilities|Array|MakeArray (Math|Conversions|ToInteger(Boolean) (Variables|Default|GetbCatchOnAir)))))
  (Ability|SendGameplayEventtoActor Owner "(TagName=\"Parkour.Climb\")" (Utilities|Struct|MakeGameplayEventData _returnvalue)))

(event EventOnStartPreparing
  (params (Owner :type Actor%20Object%20Reference))
  (Variables|Default|SetParkourHighChance 1))

(event EventOnEndPreparing
  (params (Owner :type Actor%20Object%20Reference)))

(fn PrepareParkour
  (params (StateOwner :type Actor%20Object%20Reference) (DeltaTime :type Float%20%28single-precision%29))
  (bind _returnvalue (Transformation|GetActorLocation StateOwner))
  (bind _returnvalue_2 (+ _returnvalue "0.000000,0.000000,40.000000"))
  (if (> (Variables|Default|GetParkourHighChance) 0)
    (Math|Integer|DecrementInt (Variables|Default|GetParkourHighChance)
      (:%20%20
        (LocalVariables|SetLocalCheckDistance (select (> (Math|Vector|VectorLengthXY (Transformation|GetVelocity StateOwner)) 5e+02) (Variables|Default|GetWallCheckDistanceOnRun) (Variables|Default|GetWallCheckDistanceOnWalk)))
        (Variables|Default|SetbCatchOnAir false)
        (LocalVariables|SetLocalCheckHeight (Variables|Default|GetClimbableHeight))))
    (else
      (Variables|Default|SetbCatchOnAir true)
      (LocalVariables|SetLocalCheckDistance 2e+01)
      (LocalVariables|SetLocalCheckHeight (/ (Variables|Default|GetClimbableHeight) 1.5))))
  (Utilities|FlowControl|Sequence
    (:then_0
      (bind (_outhit _returnvalue_3) (Collision|SphereTraceByChannel _returnvalue_2 (+ _returnvalue_2 (* (Transformation|GetActorForwardVector StateOwner) (LocalVariables|GetLocalCheckDistance))) 5e+01 "TraceTypeQuery3" false (Utilities|Array|MakeArray StateOwner) "None" true "(R=0.000000,G=0.930000,B=0.261164,A=1.000000)"))
      (if _returnvalue_3
        (LocalVariables|SetLocalWallHitPoint (.ImpactPoint (Collision|BreakHitResult _outhit)))
        (LocalVariables|SetLocalWallDirection (Math|Conversions|ToVector(Vector2D) (Class|KismetMathLibrary|Negated2D (Math|Conversions|ToVector2D(Vector) (.ImpactNormal (Collision|BreakHitResult _outhit))))))
        (Utilities|Array|AddUnique (LocalVariables|GetLocalWall) (.HitComponent (Collision|BreakHitResult _outhit)))
        (else
          (return 0 0 false))))
    (:then_1
      (bind (_outhit_2 _returnvalue_4) (Collision|SphereTraceByChannel (+ (LocalVariables|GetLocalWallHitPoint) (* (LocalVariables|GetLocalWallDirection) 35.0) (Math|Vector|MakeVector 0.0 0.0 (LocalVariables|GetLocalCheckHeight))) (+ (+ (LocalVariables|GetLocalWallHitPoint) (* (LocalVariables|GetLocalWallDirection) 35.0) (Math|Vector|MakeVector 0.0 0.0 (LocalVariables|GetLocalCheckHeight))) (Math|Vector|MakeVector 0.0 0.0 (* (LocalVariables|GetLocalCheckHeight) -1.0))) 35.0 "TraceTypeQuery3" false (Utilities|Array|MakeArray StateOwner) "None" true "(R=0.000000,G=0.930000,B=0.261164,A=1.000000)"))
      (if _returnvalue_4
        (if (>= (.Distance (Collision|BreakHitResult _outhit_2)) 3e+01)
          (if (<= (.Distance (Collision|BreakHitResult _outhit_2)) (- (LocalVariables|GetLocalCheckHeight) (Variables|Default|GetClimbableMinHeight)))
            (Utilities|FlowControl|Sequence
              (:then_0
                (LocalVariables|SetLocalHandPoint (+ (.ImpactPoint (Collision|BreakHitResult _outhit_2)) (* (LocalVariables|GetLocalWallDirection) -3e+01)))
                (LocalVariables|SetLocalLandPoint (.ImpactPoint (Collision|BreakHitResult _outhit_2)))
                (Utilities|Array|AddUnique (LocalVariables|GetLocalWall) (.HitComponent (Collision|BreakHitResult _outhit_2))))
              (:then_1
                (LocalVariables|SetLocalWallHitPoint (Math|Vector|MakeVector (.x (LocalVariables|GetLocalWallHitPoint)) (.y (LocalVariables|GetLocalWallHitPoint)) (- (.z (LocalVariables|GetLocalHandPoint)) 165.0)))))
            (else
              (return 0 0 false)))
          (else
            (return 0 0 false)))
        (else
          (return 0 0 false))))
    (:then_2
      (return (Utilities|Array|MakeArray (+ (LocalVariables|GetLocalWallHitPoint) (* (LocalVariables|GetLocalWallDirection) -55.0)) (LocalVariables|GetLocalHandPoint) (LocalVariables|GetLocalLandPoint) (LocalVariables|GetLocalWallDirection)) (LocalVariables|GetLocalWall) true))))