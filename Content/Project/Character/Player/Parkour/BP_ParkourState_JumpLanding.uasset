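; Parkour state for jump landings, which plays a roll or in-place landing after a long enough fall.
; On start it records the start location and triggers a parkour jump ability if the character rises at speed with open space ahead and below.
; While falling past LandingHeight, a downward trace detects ground and yields a forward landing point.
; DoParkour activates the ability and sends it the montage, chosen by velocity, via gameplay event.
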(event EventOnStartPreparing
  (params (Owner :type Actor%20Object%20Reference))
  (bind _returnvalue (Transformation|GetActorLocation Owner))
  (Variables|Default|SetInitialLocationOnStart (Transformation|GetActorLocation Owner))
  (if (and (>= (.X (Math|Vector|BreakVector (Math|Vector|UnrotateVector (Transformation|GetVelocity Owner) (Transformation|GetActorRotation Owner)))) 4e+02) (> (.z (Transformation|GetVelocity Owner)) 0.0))
    (bind (_outhit _returnvalue_2) (Collision|SphereTraceByChannel _returnvalue (+ _returnvalue (* (Transformation|GetActorForwardVector Owner) 5e+02)) 5e+01 "TraceTypeQuery1" false 0 "None"))
    (if (not _returnvalue_2)
      (bind _returnvalue_3 (Collision|SphereTraceByChannel (.TraceEnd (Collision|BreakHitResult _outhit)) (+ (.TraceEnd (Collision|BreakHitResult _outhit)) "0.000000,0.000000,-250.000000") 5e+01 "TraceTypeQuery1" false 0 "None"))
      (if (not _returnvalue_3)
        (Abilities|TryActivateAbilitybyClass (Ability|GetAbilitySystemComponent Owner) "/Game/Project/GAS/Action/Parkour/BP_STGA_ParkourJump.BP_STGA_ParkourJump_C" true)))))

(event EventDoParkour
  (params (Owner :type Actor%20Object%20Reference) (ParkourPoints :type Array%20of%20Vectors) (WallsToIgnore :type Array%20of%20Primitive%20Component%20Object%20References))
  (Abilities|TryActivateAbilitybyClass (Ability|GetAbilitySystemComponent Owner) (Variables|Default|GetParkourGA) true)
  (bind _returnvalue (Game|ConstructObjectfromClass Owner "/Game/Project/Character/Player/Parkour/BP_ParkourData.BP_ParkourData_C" ParkourPoints 0 (select (and (> (Math|Vector|VectorLengthXY (Transformation|GetVelocity Owner)) 1.5e+02) (< (Class|KismetMathLibrary|DegAcos (Class|KismetMathLibrary|VectorCosineAngle2D (Class|KismetMathLibrary|VectorNormal2D (Transformation|GetVelocity Owner) 0.0001) (Class|KismetMathLibrary|VectorNormal2D (Math|Rotator|GetRotationXVector (Transformation|GetActorRotation Owner)) 0.0001))) 15.0)) "/Game/Project/Character/Animation/ProcessedAnimation/Parkour/JumpLanding/Parkour_JumpLanding_Roll_Montage.Parkour_JumpLanding_Roll_Montage" "/Game/Project/Character/Animation/ProcessedAnimation/Parkour/JumpLanding/Parkour_JumpLanding_InPlace_Montage.Parkour_JumpLanding_InPlace_Montage")))
  (Ability|SendGameplayEventtoActor Owner "(TagName=\"Parkour.JumpLanding\")" (Utilities|Struct|MakeGameplayEventData _returnvalue)))

(event EventOnEndPreparing
  (params (Owner :type Actor%20Object%20Reference))
  (Variables|Default|SetInitialLocationOnStart "0, 0, 0"))

(fn PrepareParkour
  (params (StateOwner :type Actor%20Object%20Reference) (DeltaTime :type Float%20%28single-precision%29))
  (bind _returnvalue (Transformation|GetActorForwardVector StateOwner))
  (bind _returnvalue_2 (Transformation|GetVelocity StateOwner))
  (bind _returnvalue_3 (Math|Vector|Normalize _returnvalue))
  (bind _returnvalue_4 (/ _returnvalue_2 2.25))
  (bind _returnvalue_5 (* _returnvalue_3 2.5e+02))
  (LocalVariables|SetLocalCurrentLoc (Transformation|GetActorLocation StateOwner))
  (if (< (.Z (Math|Vector|BreakVector (Transformation|GetVelocity StateOwner))) 0.0)
    (if (> (- (.z (Variables|Default|GetInitialLocationOnStart)) (.z (LocalVariables|GetLocalCurrentLoc))) (Variables|Default|GetLandingHeight))
      (bind _returnvalue_6 (Collision|LineTraceByChannel (LocalVariables|GetLocalCurrentLoc) (+ (LocalVariables|GetLocalCurrentLoc) "0.000000,0.000000,-125.000000") "TraceTypeQuery1" false 0 "None" true "(R=1.000000,G=0.000000,B=0.000000,A=1.000000)" "(R=0.000000,G=1.000000,B=0.000000,A=1.000000)" 1.0))
      (if _returnvalue_6
        (return (Utilities|Array|MakeArray (+ (Transformation|GetActorLocation StateOwner) (select (> (Math|Vector|VectorLengthXY _returnvalue_5) (Math|Vector|VectorLengthXY _returnvalue_4)) _returnvalue_5 _returnvalue_4))) 0 true)))))