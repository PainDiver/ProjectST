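; Parkour state that detects a mantle over a ledge in front of the character and triggers it through GAS.
; PrepareParkour chains sphere traces to find the wall at a speed-dependent distance, the ledge top, clear space beyond and nearby ground to land on.
; It outputs wall direction, approach and hand points, plus walls to ignore.
; DoParkour activates the parkour ability, then sends these with the montage in a Parkour.Mantle gameplay event.
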(event EventDoParkour
  (params (Owner :type Actor%20Object%20Reference) (ParkourPoints :type Array%20of%20Vectors) (WallsToIgnore :type Array%20of%20Primitive%20Component%20Object%20References))
  (Abilities|TryActivateAbilitybyClass (Ability|GetAbilitySystemComponent Owner) (Variables|Default|GetParkourGA) true)
  (bind _returnvalue (Game|ConstructObjectfromClass Owner "/Game/Project/Character/Player/Parkour/BP_ParkourData.BP_ParkourData_C" ParkourPoints WallsToIgnore "/Game/Project/Character/Animation/ProcessedAnimation/Parkour/Mantle/Parkour_Mantle_Run.Parkour_Mantle_Run"))
  (Ability|SendGameplayEventtoActor Owner "(TagName=\"Parkour.Mantle\")" (Utilities|Struct|MakeGameplayEventData _returnvalue)))

(fn PrepareParkour
  (params (StateOwner :type Actor%20Object%20Reference) (DeltaTime :type Float%20%28single-precision%29))
  (bind _returnvalue (Transformation|GetActorLocation StateOwner))
  (bind _returnvalue_2 (+ _returnvalue ""))
  (LocalVariables|SetLocalIsRunning (> (Math|Vector|VectorLengthXY (Transformation|GetVelocity StateOwner)) 5e+02))
  (LocalVariables|SetLocalWallCheckDistance (select (LocalVariables|GetLocalIsRunning) (Variables|Default|GetWallCheckDistanceOnWalk) (Variables|Default|GetWallCheckDistanceOnRun)))
  (Utilities|FlowControl|Sequence
    (:then_0
      (bind (_outhit _returnvalue_3) (Collision|SphereTraceByChannel _returnvalue_2 (+ _returnvalue_2 (* (Transformation|GetActorForwardVector StateOwner) (LocalVariables|GetLocalWallCheckDistance))) 35.0 "TraceTypeQuery3" false (Utilities|Array|MakeArray StateOwner) "None" true "(R=0.000000,G=0.930000,B=0.261164,A=1.000000)"))
      (if _returnvalue_3
        (LocalVariables|SetLocalHorizontalPoint (.ImpactPoint (Collision|BreakHitResult _outhit)))
        (LocalVariables|SetLocalWallDirection (Class|KismetMathLibrary|VectorNormal2D (Math|Vector|NegateVector (.ImpactNormal (Collision|BreakHitResult _outhit))) 0.0001))
        (Utilities|Array|AddUnique (LocalVariables|GetLocalIgnoredWalls) (.HitComponent (Collision|BreakHitResult _outhit)))
        (else
          (return 0 0 false))))
    (:then_1
      (bind (_outhit_2 _returnvalue_4) (Collision|SphereTraceByChannel (+ (LocalVariables|GetLocalHorizontalPoint) (* (LocalVariables|GetLocalWallDirection) 25.0) "0.000000,0.000000,125.000000") (+ (+ (LocalVariables|GetLocalHorizontalPoint) (* (LocalVariables|GetLocalWallDirection) 25.0) "0.000000,0.000000,125.000000") "0.000000,0.000000,-200.000000") 35.0 "TraceTypeQuery3" false (Utilities|Array|MakeArray StateOwner) "None"))
      (if _returnvalue_4
        (if (>= (.Distance (Collision|BreakHitResult _outhit_2)) 3e+01)
          (LocalVariables|SetLocalHandPoint (.ImpactPoint (Collision|BreakHitResult _outhit_2)))
          (Utilities|Array|AddUnique (LocalVariables|GetLocalIgnoredWalls) (.HitComponent (Collision|BreakHitResult _outhit_2))))
        (else
          (return 0 0 false))))
    (:then_2
      (bind (_outhit_3 _returnvalue_5) (Collision|SphereTraceByChannel (+ (LocalVariables|GetLocalHandPoint) "0.000000,0.000000,25.000000") (+ (LocalVariables|GetLocalHandPoint) (* (LocalVariables|GetLocalWallDirection) 1.5e+02) "0.000000,0.000000,25.000000") 15.0 "TraceTypeQuery3" false (Utilities|Array|MakeArray StateOwner) "None"))
      (if _returnvalue_5
        (return 0 0 false)
        (else
          (bind (_outhit_4 _returnvalue_6) (Collision|SphereTraceByChannel (.TraceEnd (Collision|BreakHitResult _outhit_3)) (+ (.TraceEnd (Collision|BreakHitResult _outhit_3)) "0.000000,0.000000,-200.000000") 2e+01 "TraceTypeQuery3" false (Utilities|Array|MakeArray StateOwner) "None"))
          (if _returnvalue_6
            (if (not (<= (.Distance (Collision|BreakHitResult _outhit_4)) 1e+02))
              (return 0 0 false))
            (else
              (return 0 0 false))))))
    (:then_3
      (return (Utilities|Array|MakeArray (LocalVariables|GetLocalWallDirection) (+ (LocalVariables|GetLocalHorizontalPoint) (* (LocalVariables|GetLocalWallDirection) -7e+01)) (LocalVariables|GetLocalHandPoint)) (LocalVariables|GetLocalIgnoredWalls) true))))