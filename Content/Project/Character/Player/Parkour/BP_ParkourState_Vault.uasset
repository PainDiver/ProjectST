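; Parkour state for vaulting: detects a vaultable obstacle ahead of the character and triggers the vault through GAS.
; PrepareParkour chains sphere traces to find the obstacle face, a hand point on top and an air point beyond, collecting walls to ignore.
; DoParkour activates the parkour ability, then sends it a Parkour.Vault event carrying the hand and air points, ignored walls and a close or far montage chosen by distance.
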(event EventDoParkour
  (params (Owner :type Actor%20Object%20Reference) (ParkourPoints :type Array%20of%20Vectors) (WallsToIgnore :type Array%20of%20Primitive%20Component%20Object%20References))
  (bind _output (Utilities|Array|Get(acopy) ParkourPoints 2))
  (Abilities|TryActivateAbilitybyClass (Ability|GetAbilitySystemComponent Owner) (Variables|Default|GetParkourGA) true)
  (bind _returnvalue (Game|ConstructObjectfromClass Owner "/Game/Project/Character/Player/Parkour/BP_ParkourData.BP_ParkourData_C" (Utilities|Array|MakeArray (Utilities|Array|Get(acopy) ParkourPoints 1) _output) WallsToIgnore (select (and (< (Math|Vector|Distance2D(Vector) _output (Transformation|GetActorLocation Owner)) 1.5e+02) (< (Math|Vector|Distance2D(Vector) (Utilities|Array|Get(acopy) ParkourPoints) (Transformation|GetActorLocation Owner)) 1e+02)) "/Game/Project/Character/Animation/ProcessedAnimation/Parkour/Vault/Parkour_Vault_Close.Parkour_Vault_Close" "/Game/Project/Character/Animation/ProcessedAnimation/Parkour/Vault/Parkour_Vault_Far.Parkour_Vault_Far")))
  (Ability|SendGameplayEventtoActor Owner "(TagName=\"Parkour.Vault\")" (Utilities|Struct|MakeGameplayEventData _returnvalue)))

(event EventOnEndPreparing
  (params (Owner :type Actor%20Object%20Reference)))

(event EventOnStartPreparing
  (params (Owner :type Actor%20Object%20Reference)))

(fn PrepareParkour
  (params (StateOwner :type Actor%20Object%20Reference) (DeltaTime :type Float%20%28single-precision%29))
  (bind _returnvalue (Transformation|GetActorLocation StateOwner))
  (bind _returnvalue_2 (+ _returnvalue "0.000000,0.000000,-40.000000"))
  (Utilities|FlowControl|Sequence
    (:then_0
      (bind (_outhit _returnvalue_3) (Collision|SphereTraceByChannel _returnvalue_2 (+ _returnvalue_2 (* (Transformation|GetActorForwardVector StateOwner) 175.0)) 35.0 "TraceTypeQuery3" false (Utilities|Array|MakeArray StateOwner) "None" true "(R=0.000000,G=0.930000,B=0.261164,A=1.000000)"))
      (if _returnvalue_3
        (LocalVariables|SetLocalHorizontalPoint (.ImpactPoint (Collision|BreakHitResult _outhit)))
        (Utilities|Array|AddUnique (LocalVariables|GetLocalIgnoredWalls) (.HitComponent (Collision|BreakHitResult _outhit)))
        (else
          (return 0 0 false))))
    (:then_1
      (bind (_outhit_2 _returnvalue_4) (Collision|SphereTraceByChannel (+ (LocalVariables|GetLocalHorizontalPoint) (* (Transformation|GetActorForwardVector StateOwner) 5e+01) "0.000000,0.000000,150.000000") (+ (+ (LocalVariables|GetLocalHorizontalPoint) (* (Transformation|GetActorForwardVector StateOwner) 5e+01) "0.000000,0.000000,150.000000") "0.000000,0.000000,-150.000000") 35.0 "TraceTypeQuery3" false (Utilities|Array|MakeArray StateOwner) "None"))
      (if _returnvalue_4
        (if (>= (.Distance (Collision|BreakHitResult _outhit_2)) 5e+01)
          (LocalVariables|SetLocalHandPoint (+ (.ImpactPoint (Collision|BreakHitResult _outhit_2)) "0.000000,0.000000,25.000000"))
          (Utilities|Array|AddUnique (LocalVariables|GetLocalIgnoredWalls) (.HitComponent (Collision|BreakHitResult _outhit_2)))
          (else
            (return 0 0 false)))
        (else
          (return 0 0 false))))
    (:then_2
      (bind (_outhit_3 _returnvalue_5) (Collision|SphereTraceByChannel (+ (LocalVariables|GetLocalHandPoint) "0.000000,0.000000,25.000000") (+ (+ (LocalVariables|GetLocalHandPoint) "0.000000,0.000000,25.000000") (* (Transformation|GetActorForwardVector StateOwner) 3e+02)) 35.0 "TraceTypeQuery3" false (Utilities|Array|MakeArray StateOwner) "None"))
      (if _returnvalue_5
        (if (>= (.Distance (Collision|BreakHitResult _outhit_3)) 2.5e+02)
          (LocalVariables|SetLocalAirPoint (+ (.ImpactPoint (Collision|BreakHitResult _outhit_3)) (* (Transformation|GetActorForwardVector StateOwner) -5e+01)))
          (Utilities|Array|AddUnique (LocalVariables|GetLocalIgnoredWalls) (.HitComponent (Collision|BreakHitResult _outhit_3)))
          (else
            (return 0 0 false)))
        (else
          (bind (_outhit_4 _returnvalue_6) (Collision|SphereTraceByChannel (+ (.TraceEnd (Collision|BreakHitResult _outhit_3)) "0.000000,0.000000,-50.000000") (+ (+ (.TraceEnd (Collision|BreakHitResult _outhit_3)) "0.000000,0.000000,-50.000000") (* (Transformation|GetActorForwardVector StateOwner) -3e+02)) 35.0 "TraceTypeQuery3" false 0 "None" true "(R=0.984931,G=1.000000,B=0.450000,A=1.000000)"))
          (if _returnvalue_6
            (LocalVariables|SetLocalAirPoint (+ (* (Transformation|GetActorForwardVector StateOwner) 5e+01) (.ImpactPoint (Collision|BreakHitResult _outhit_4))))
            (else
              (return 0 0 false))))))
    (:then_3
      (return (Utilities|Array|MakeArray (LocalVariables|GetLocalHorizontalPoint) (LocalVariables|GetLocalHandPoint) (LocalVariables|GetLocalAirPoint)) (LocalVariables|GetLocalIgnoredWalls) true))))