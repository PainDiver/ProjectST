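; Player controller, named for the login stage, that runs startup initialization behind a loading fade.
; On BeginPlay, Initialize has the HUD fade in instantly with a loading indicator, initializes the interface message, and calls ForceStreamingLoadAndCompile on the game instance.
; The same Sequence then starts a timed fade-out without the indicator.
; A hardcoded test login through the STNetManager packet handler is left unconnected, along with its debug-print response event.
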(event Custom|커스텀이벤트
  (params (Message :type SC%20Packet%20Login%20Structure%20%28by%20ref%29))
  (Development|PrintString (Utilities|String|ToString(Boolean) false)))

(event EventBeginPlay
  (CallFunction|Initialize))

(event EventTick
  (params (DeltaSeconds :type Float%20%28single-precision%29)))

(fn ConstructionScript)

(fn Initialize
  (Utilities|FlowControl|Sequence
    (:then_0
      (Class|IBPSTHUDInterface|FadeinOutInterface(Message) (HUD|GetHUD) true 0.0 true))
    (:then_1
      (Class|IBPSTHUDInterface|InitializeInterface(Message) (HUD|GetHUD))
      (bind _returnvalue (Class|STGameBlueprintFunctionLibrary|GetSTGameInstance))
      (Class|STGameInstance|ForceStreamingLoadandCompile _returnvalue))
    (:then_2
      (Class|IBPSTHUDInterface|FadeinOutInterface(Message) (HUD|GetHUD) false 1.0 false))))