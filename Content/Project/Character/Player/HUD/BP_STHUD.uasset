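; Player HUD Blueprint that owns the in-game base widget and acts as the entry point for gameplay UI updates.
; On initialization it waits once for the pawn's CharacterPrepared event, then creates, registers and shows the base widget with a HUD widget controller.
; Cooldown, skill, vital and message calls forward to that widget via tag lookup.
; Screen fades use a separate, lazily created widget at a high viewport Z-order.
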(event Custom|OnInit
  (params (Data :type Object%20Object%20Reference))
  (bind _returnvalue (Game|Player|GetOwningPlayerController))
  (Utilities|FlowControl|Sequence
    (:then_0
      (bind _returnvalue_2 (UserInterface|CreateWidget "/Game/Project/UI/InGame/Base/HUDBase/STWBP_InGameBase.STWBP_InGameBase_C" _returnvalue))
      (bind _returnvalue_3 (Game|ConstructObjectfromClass _returnvalue "/Script/ProjectST.STWidgetController_HUD"))
      (Class|STHUD|RegisterWidget "(TagName=\"UI.HUDBase\")" _returnvalue_2 _returnvalue_3)
      (Class|STHUD|ShowWidget "(TagName=\"UI.HUDBase\")")
      (Default|Initialize _returnvalue_2))))

(event EventBeginPlay)

(event Collision|EventActorBeginOverlap
  (params (OtherActor :type Actor%20Object%20Reference)))

(event EventTick
  (params (DeltaSeconds :type Float%20%28single-precision%29)))

(event EventInitializeInterface
  (Class|STEventManager|RegisterEventSubject (Subsystems|GetSTEventManager) (Class|HUD|GetOwningPawn) "(TagName=\"Event.CharacterPrepared\")" (delegate Custom|OnInit) 0 true))

(fn ConstructionScript)

(fn FadeinOutInterface
  (params (FadeIn :type Boolean) (Time :type Float%20%28double-precision%29) (ShowLoading :type Boolean))
  (Utilities|IsValid (Variables|Default|GetFadeWidget)
    (:Is%20Valid
      (Default|FadeinOut (Variables|Default|GetFadeWidget) FadeIn Time ShowLoading))
    (:Is%20Not%20Valid
      (bind _returnvalue (UserInterface|CreateWidget "/Game/Project/UI/PopUp/WBP_FadeInOut.WBP_FadeInOut_C" (Game|GetPlayerController 0)))
      (bind _output_get (Variables|Default|SetFadeWidget _returnvalue))
      (UserInterface|Viewport|AddtoViewport _output_get 9999)
      (Default|FadeinOut _output_get FadeIn Time ShowLoading))))

(fn SetCoolTime
  (params (GA :type Gameplay%20Ability%20Object%20Reference))
  (bind _returnvalue (Class|STHUD|GetWidgetbyTag "(TagName=\"UI.HUDBase\")"))
  (bind _asstwbp_in_game_base (Utilities|Casting|CastToSTWBP_InGameBase _returnvalue))
  (Default|UpdateCooltime _asstwbp_in_game_base GA))

(fn ShowMessage
  (params (MessageType :type SystemMessageType%20Enum :default "NewEnumerator0") (Text :type Text))
  (bind _returnvalue (Class|STHUD|GetWidgetbyTag "(TagName=\"UI.HUDBase\")"))
  (bind _asstwbp_in_game_base (Utilities|Casting|CastToSTWBP_InGameBase _returnvalue))
  (Default|ShowMessage _asstwbp_in_game_base MessageType Text)
  (return true))

(fn UpdateSkill
  (bind _returnvalue (Class|STHUD|GetWidgetbyTag "(TagName=\"UI.HUDBase\")"))
  (bind _asstwbp_in_game_base (Utilities|Casting|CastToSTWBP_InGameBase _returnvalue))
  (Default|UpdateSkills _asstwbp_in_game_base)
  (return true))

(fn UpdateVitalInterface
  (params (VitalType :type EVitalType%20Enum :default "NewEnumerator0") (Percent :type Float%20%28double-precision%29))
  (bind _returnvalue (Class|STHUD|GetWidgetbyTag "(TagName=\"UI.HUDBase\")"))
  (bind _asstwbp_in_game_base (Utilities|Casting|CastToSTWBP_InGameBase _returnvalue))
  (Default|UpdateVital _asstwbp_in_game_base VitalType Percent)
  (return true))