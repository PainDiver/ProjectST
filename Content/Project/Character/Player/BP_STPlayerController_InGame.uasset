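; In-game player controller that routes typed text messages to the player's HUD.
; On BeginPlay, only the local controller initializes the HUD through an interface message.
; Message interface events either show text on the HUD directly or go through a client-named event intended for the owning player's HUD.
; The interactable scan callback and Tick are empty.
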(event Custom|ShowMessage_Client
  (params (MessageType :type SystemMessageType%20Enum :default "NewEnumerator0") (Text :type Text))
  (Class|IBPSTHUDInterface|ShowMessage(Message) (HUD|GetHUD) MessageType Text))

(event EventBeginPlay
  (CallFunction|Initialize))

(event EventTick
  (params (DeltaSeconds :type Float%20%28single-precision%29)))

(event EventShowMessageInterface
  (params (MessageType :type SystemMessageType%20Enum :default "NewEnumerator0") (Message :type Text))
  (Class|IBPSTHUDInterface|ShowMessage(Message) (HUD|GetHUD) MessageType Message))

(event EventShowMessageClientInterface
  (params (Type :type SystemMessageType%20Enum :default "NewEnumerator0") (Text :type Text))
  (CallFunction|ShowMessageClient Type Text))

(fn ConstructionScript)

(fn Initialize
  (Utilities|FlowControl|Sequence
    (:then_0
      (if (Pawn|IsLocalPlayerController)
        (Class|IBPSTHUDInterface|InitializeInterface(Message) (HUD|GetHUD))))))

(fn OnScanNewInteractableObject
  (params (OldScannedActor :type Actor%20Object%20Reference) (NewScannedActor :type Actor%20Object%20Reference)))