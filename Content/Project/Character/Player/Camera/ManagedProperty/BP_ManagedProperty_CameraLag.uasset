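; Managed camera property that drives the player spring arm's camera lag speed from the character's velocity.
; The float target update maps velocity magnitude through a clamped range, so the lag speed value rises as the character moves faster.
; The post-update event then interpolates the spring arm's CameraLagSpeed toward that target at the configured interp speed.
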(event EventPostUpdateTargetFloat
  (params (Character :type ST%20Player%20Character%20Object%20Reference) (Camera :type Camera%20Component%20Object%20Reference) (SpringArm :type Spring%20Arm%20Component%20Object%20Reference) (Target :type Float%20%28single-precision%29) (DeltaTime :type Float%20%28single-precision%29))
  (Variables|/Script/Engine.SpringArmComponent|SetCameraLagSpeed SpringArm (Math|Interpolation|FInterpTo (Variables|/Script/Engine.SpringArmComponent|GetCameraLagSpeed SpringArm) Target DeltaTime (Variables|Default|GetInterp%20Speed))))

(fn UpdateTargetFloat
  (params (Character :type ST%20Player%20Character%20Object%20Reference) (Camera :type Camera%20Component%20Object%20Reference) (SpringArm :type Spring%20Arm%20Component%20Object%20Reference) (DeltaTime :type Float%20%28single-precision%29))
  (Utilities|FlowControl|Sequence
    (:then_0
      (return (Math|Float|MapRangeClamped (Math|Vector|VectorLength (Transformation|GetVelocity Character)) 0.0 1e+03 0.0 35.0)))))