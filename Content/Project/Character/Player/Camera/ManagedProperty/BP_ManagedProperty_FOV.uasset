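; Managed camera property that drives the player camera's field of view from character movement speed.
; UpdateTargetFloat maps the character's velocity length through a clamped range to a target FOV, widening the view as speed rises.
; PostUpdateTargetFloat then eases the camera's current FOV toward that target with FInterpTo at a configurable interpolation speed.
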(event EventPostUpdateTargetFloat
  (params (Character :type ST%20Player%20Character%20Object%20Reference) (Camera :type Camera%20Component%20Object%20Reference) (SpringArm :type Spring%20Arm%20Component%20Object%20Reference) (Target :type Float%20%28single-precision%29) (DeltaTime :type Float%20%28single-precision%29))
  (Variables|/Script/Engine.CameraComponent|SetFieldOfView Camera (Math|Interpolation|FInterpTo (Variables|/Script/Engine.CameraComponent|GetFieldOfView Camera) Target DeltaTime (Variables|Default|GetInterp%20Speed))))

(fn UpdateTargetFloat
  (params (Character :type ST%20Player%20Character%20Object%20Reference) (Camera :type Camera%20Component%20Object%20Reference) (SpringArm :type Spring%20Arm%20Component%20Object%20Reference) (DeltaTime :type Float%20%28single-precision%29))
  (Utilities|FlowControl|Sequence
    (:then_1
      (return (Math|Float|MapRangeClamped (Math|Vector|VectorLength (Transformation|GetVelocity Character)) 0.0 1.2e+03 85.0 115.0)))))