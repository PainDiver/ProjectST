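; Managed camera property that eases the player camera's aspect ratio back to 16:9.
; The target update always returns 16:9 and switches off the aspect ratio constraint once a constrained camera's ratio has narrowed to a threshold slightly wider than that.
; The post-update event then interpolates the camera's current ratio toward the target using FInterpTo at the configured speed.
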(event EventPostUpdateTargetFloat
  (params (Character :type ST%20Player%20Character%20Object%20Reference) (Camera :type Camera%20Component%20Object%20Reference) (SpringArm :type Spring%20Arm%20Component%20Object%20Reference) (Target :type Float%20%28single-precision%29) (DeltaTime :type Float%20%28single-precision%29))
  (Class|CameraComponent|SetAspectRatio Camera (Math|Interpolation|FInterpTo (Variables|/Script/Engine.CameraComponent|GetAspectRatio Camera) Target DeltaTime (Variables|Default|GetInterp%20Speed))))

(fn UpdateTargetFloat
  (params (Character :type ST%20Player%20Character%20Object%20Reference) (Camera :type Camera%20Component%20Object%20Reference) (SpringArm :type Spring%20Arm%20Component%20Object%20Reference) (DeltaTime :type Float%20%28single-precision%29))
  (Utilities|FlowControl|Sequence
    (:then_0
      (if (Variables|/Script/Engine.CameraComponent|GetbConstrainAspectRatio Camera)
        (if (<= (Variables|/Script/Engine.CameraComponent|GetAspectRatio Camera) 1.95)
          (Variables|/Script/Engine.CameraComponent|SetbConstrainAspectRatio Camera false))))
    (:then_1
      (return 1.777778))))