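; Functional test that checks whether the GameState can create a dropped field item.
; On authority, after a short delay, it finds the first BP_STPlayerCharacter and has STGameState spawn an item actor at that location via CreateItemActor.
; A valid actor is passed to CheckClient1, intended as the client replication check, which finishes the test on its validity.
; Failed creation fails the test, while failed PlayerState or GameState casts stop without finishing.
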(event Custom|CheckClient1
  (params (Dropped :type Actor%20Object%20Reference))
  ;[0.15 0.15 0.15 0.5] GameState_CreateFieldItem - GameState Creates Item and replicate to Client
  (Utilities|IsValid Dropped
    (:Is%20Valid
      (Class|FunctionalTest|FinishTest "Succeeded" "Field Item Succeesfully Dropped"))
    (:Is%20Not%20Valid
      (Class|FunctionalTest|FinishTest "Failed" "Field Item Not Dropped On Client"))))

(event EventPrepareTest)

(event EventStartTest
  ;[0.15 0.15 0.15 0.5] GameState_CreateFieldItem - GameState Creates Item and replicate to Client
  (if (Ability|HasAuthority)
    (Utilities|FlowControl|Delay 2.0)
    (bind _outactors (Actor|GetAllActorsOfClass "/Game/Project/Character/Player/BP_STPlayerCharacter.BP_STPlayerCharacter_C"))
    (bind _output_get (Variables|Default|SetCharacter (Utilities|Array|Get(acopy) _outactors)))
    (Utilities|Casting|CastToSTPlayerState (Variables|/Script/Engine.Pawn|GetPlayerState _output_get))
    (bind _asstgame_state (Utilities|Casting|CastToSTGameState (Game|GetGameState)))
    (bind _returnvalue (Class|STGameState|CreateItemActor _asstgame_state 1 (Transformation|GetActorLocation _output_get) "0, 0, 0" 1))
    (Utilities|IsValid _returnvalue
      (:Is%20Valid
        (Development|PrintString "Field Item Dropped")
        (CallFunction|CheckClient1 _returnvalue))
      (:Is%20Not%20Valid
        (Development|PrintString "Field Item Not Created")
        (Class|FunctionalTest|FinishTest "Failed" "Field Item Not Dropped On Server")))))

(event EventTick
  (params (DeltaSeconds :type Float%20%28single-precision%29)))

(fn ConstructionScript)