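; Functional test that checks the GameState can create an item directly in a player's inventory.
; On authority, after a short delay, it takes the first BP_STPlayerCharacter and calls CreateItemObjectToOwner on STGameState, targeting that PlayerState's InventoryComponent.
; If creation succeeds, CheckClient2 reads the first inventory slot and passes or fails the test on its item ID.
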(event Custom|CheckClient2
  (params (Character :type Actor%20Object%20Reference))
  ;[0.15 0.15 0.15 0.5] GameState_GiveItem - GameState Creates Item and put in the inventory
  (bind _as캐릭터 (Utilities|Casting|CastToCharacter Character))
  (bind _asstplayer_state (Utilities|Casting|CastToSTPlayerState (Variables|/Script/Engine.Pawn|GetPlayerState _as캐릭터)))
  (Utilities|Casting|CastToSTGameState (Game|GetGameState))
  (if (== (.ItemID (Utilities|Struct|BreakReplicatedItemData (Utilities|Array|Get(acopy) (Utilities|Struct|BreakInventoryContainer (Class|STInventoryComponent|GetInventoryComponent (Variables|/Script/ProjectST.STPlayerState|GetInventoryComponent _asstplayer_state)))))) 1)
    (Development|PrintString (Utilities|String|Append "New Item GUID : " (Guid|ToString(Guid) (.ItemUID (Utilities|Struct|BreakReplicatedItemData (Utilities|Array|Get(acopy) (Utilities|Struct|BreakInventoryContainer (Class|STInventoryComponent|GetInventoryComponent (Variables|/Script/ProjectST.STPlayerState|GetInventoryComponent _asstplayer_state)))))))))
    (Class|FunctionalTest|FinishTest "Succeeded" "Item Succeesfully Given To Owner")
    (else
      (Class|FunctionalTest|FinishTest "Failed" "Field Item Not Dropped On Client"))))

(event EventPrepareTest)

(event EventStartTest
  ;[0.15 0.15 0.15 0.5] GameState_GiveItem - GameState Creates Item and put in the inventory
  (if (Ability|HasAuthority)
    (Utilities|FlowControl|Delay 2.0)
    (bind _outactors (Actor|GetAllActorsOfClass "/Game/Project/Character/Player/Classes/BP_STPlayerCharacter.BP_STPlayerCharacter_C"))
    (bind _output_get (Variables|Default|SetCharacter (Utilities|Array|Get(acopy) _outactors)))
    (bind _asstplayer_state (Utilities|Casting|CastToSTPlayerState (Variables|/Script/Engine.Pawn|GetPlayerState _output_get)))
    (bind _asstgame_state (Utilities|Casting|CastToSTGameState (Game|GetGameState)))
    (bind _returnvalue (Class|STGameState|CreateItemObjecttoOwner _asstgame_state 1 1 (Variables|/Script/ProjectST.STPlayerState|GetInventoryComponent _asstplayer_state) "INVENTORY"))
    (if _returnvalue
      (Development|PrintString "Item Object Created")
      (CallFunction|CheckClient2 (Variables|Default|GetCharacter))
      (else
        (Development|PrintString "Item Object Not Created")
        (Class|FunctionalTest|FinishTest "Failed" "Item Object was not created")))))

(event EventTick
  (params (DeltaSeconds :type Float%20%28single-precision%29)))

(fn ConstructionScript)